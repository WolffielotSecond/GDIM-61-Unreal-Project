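; Character component that moves the owning third-person character through the start, middle and end phases of a vault animation.
; SetStartandEndPos stores the vault points and traces down ahead of the end point for a landing spot, reaching farther when running and falling back to the end point.
; DoTranslateCharacter selects the phase's target and duration, then Tick linearly interpolates the actor there without sweeping.
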(event Custom|Do%20Translate%20Character
  (params (Time%20DUration :type Float%20%28double-precision%29) (Is%20Start%20Animation :type Boolean) (Is%20Middle%20Animation :type Boolean) (Is%20End%20Animation :type Boolean))
  ;[0.15 0.15 0.15 0.5] 开始 中间 结尾逻辑
  (Variables|Default|SetTime%20Duration Time%20DUration)
  (if Is%20Start%20Animation
    (Variables|Default|SetStart%20Location (Transformation|GetActorLocation (Variables|Default|GetPlayer%20Ref)))
    (Variables|Default|SetTarget%20Location (Variables|Default|GetStart%20Pos))
    (Variables|Default|SetShould%20Move%20Character true)
    (Variables|Default|SetElapsed%20Time 0.0)
    (elif Is%20Middle%20Animation
      (Variables|Default|SetStart%20Location (Transformation|GetActorLocation (Variables|Default|GetPlayer%20Ref)))
      (Variables|Default|SetTarget%20Location (Variables|Default|GetEnd%20Pos))
      (Variables|Default|SetShould%20Move%20Character true)
      (Variables|Default|SetElapsed%20Time 0.0)
      (elif Is%20End%20Animation
        (Variables|Default|SetStart%20Location (Transformation|GetActorLocation (Variables|Default|GetPlayer%20Ref)))
        (Variables|Default|SetTarget%20Location (Variables|Default|GetLand%20Location))
        (Variables|Default|SetShould%20Move%20Character true)
        (Variables|Default|SetElapsed%20Time 0.0)))))

(event Custom|Set%20Start%20and%20End%20Pos
  (params (Start :type Vector) (End :type Vector) (Is%20Run :type Boolean))
  (if Is%20Run
    (Variables|Default|SetLand%20Location%20Offset 175.0)
    (else
      (Variables|Default|SetLand%20Location%20Offset 5e+01)))
  (Variables|Default|SetStart%20Pos Start)
  (bind _output_get (Variables|Default|SetEnd%20Pos End))
  (bind (_outhit _returnvalue) (Collision|LineTraceByChannel (+ (* (Math|Vector|GetForwardVector (Transformation|GetActorRotation (Variables|Default|GetPlayer%20Ref))) (Variables|Default|GetLand%20Location%20Offset)) _output_get) (+ (+ (* (Math|Vector|GetForwardVector (Transformation|GetActorRotation (Variables|Default|GetPlayer%20Ref))) (Variables|Default|GetLand%20Location%20Offset)) _output_get) (* (Math|Vector|VectorDown) 2e+02)) "TraceTypeQuery1" false 0 "None"))
  (if _returnvalue
    (Variables|Default|SetLand%20Location (+ (.Location (Collision|BreakHitResult _outhit)) (* (Math|Vector|VectorUp) 88.0)))
    (else
      (Variables|Default|SetLand%20Location (Variables|Default|GetEnd%20Pos)))))

(event EventBeginPlay
  (bind _asbp_third_person_character_base (Utilities|Casting|CastToBP_ThirdPersonCharacter_Base (Components|GetOwner)))
  (Variables|Default|SetPlayer%20Ref _asbp_third_person_character_base))

(event EventTick
  (params (DeltaSeconds :type Float%20%28single-precision%29))
  ;[0.15 0.15 0.15 0.5] 可以移动角色时移动角色
  (if (Variables|Default|GetShould%20Move%20Character)
    (Utilities|FlowControl|Sequence
      (:then_0
        (Variables|Default|SetElapsed%20Time (+ (Variables|Default|GetElapsed%20Time) (Utilities|Time|GetWorldDeltaSeconds)))
        (if (>= (Variables|Default|GetElapsed%20Time) (Variables|Default|GetTime%20Duration))
          (Variables|Default|SetShould%20Move%20Character false)))
      (:then_1
        (Transformation|SetActorLocation (Variables|Default|GetPlayer%20Ref) (Math|Vector|Lerp(Vector) (Variables|Default|GetStart%20Location) (Variables|Default|GetTarget%20Location) (Math|Float|Clamp(Float) (/ (Variables|Default|GetElapsed%20Time) (Variables|Default|GetTime%20Duration)))) false false)))))