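; BP_Meimei is a character that transforms into a boss and triggers a floor collapse sequence.
; Transform disables player input, swaps the visible mesh for the Boss component hidden at BeginPlay, and jumps.
; Landing calls a save-game message, hides the floor and removes its collision, then switches Meimei to flying.
; It also flags the collapsing sequence on the player character and enables physics simulation on a set of actors.
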(event Custom|Transform
  (Input|DisableInput (Game|GetPlayerCharacter 0) (Game|GetPlayerController 0))
  (Rendering|SetVisibility (Variables|Default|GetBoss) true true)
  (Rendering|SetVisibility (Variables|Character|GetMesh) false false)
  (Character|Jump))

(event EventBeginPlay
  (Rendering|SetVisibility (Variables|Default|GetBoss) false true))

(event EventOnLanded
  (params (Hit :type Hit%20Result%20Structure%20%28by%20ref%29))
  (bind _floor (Variables|Default|GetFloor))
  (Class|BPIGamecontroller|SaveGametoGameInstance(Message) (Game|GetPlayerController 0))
  (Rendering|SetVisibility (Variables|/Script/Engine.StaticMeshActor|GetStaticMeshComponent _floor) false false)
  (Collision|SetCollisionEnabled (Variables|/Script/Engine.StaticMeshActor|GetStaticMeshComponent _floor) "NoCollision")
  (Pawn|Components|CharacterMovement|SetMovementMode (Variables|Character|GetCharacterMovement) "MOVE_Flying" 0)
  (bind _asbp_third_person_character_base (Utilities|Casting|CastToBP_ThirdPersonCharacter_Base (Game|GetPlayerCharacter 0)))
  (Variables|/Game/Characters/BP_ThirdPersonCharacter_Base.BP_ThirdPersonCharacter_Base_C|SetTriggered%20Collapsing%20Sequence _asbp_third_person_character_base true)
  (for _array_element (Variables|Default|GetSimulate%20Physics%20Actors)
    (Physics|SetSimulatePhysics (Variables|/Script/Engine.StaticMeshActor|GetStaticMeshComponent _array_element) true)))

(fn ConstructionScript)