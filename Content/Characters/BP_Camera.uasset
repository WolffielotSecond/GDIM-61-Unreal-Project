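; BP_Camera is a camera actor that smoothly follows the player while a follow flag is set.
; Each tick it checks the player reference, then interpolates its location toward the player's CameraPrompt component with VInterpTo.
; The target keeps the prompt's world Y and Z but divides X by 100, so the camera follows only a small fraction of that axis.
; Rotation is never changed.
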(event EventBeginPlay)

(event Collision|EventActorBeginOverlap
  (params (OtherActor :type Actor%20Object%20Reference)))

(event EventTick
  (params (DeltaSeconds :type Float%20%28single-precision%29))
  (if (Variables|Default|GetCamera%20Should%20Follow%20Player)
    (bind _player_reference (Variables|Default|GetPlayer%20Reference)
      (:then
        (Transformation|SetActorLocation (Math|Interpolation|VInterpTo (Transformation|GetActorLocation) (Math|Vector|MakeVector (/ (.x (Transformation|GetWorldLocation (Variables|/Game/Characters/BP_ThirdPersonCharacter_Base.BP_ThirdPersonCharacter_Base_C|GetCamera%20Prompt _player_reference))) 1e+02) (.y (Transformation|GetWorldLocation (Variables|/Game/Characters/BP_ThirdPersonCharacter_Base.BP_ThirdPersonCharacter_Base_C|GetCamera%20Prompt _player_reference))) (.z (Transformation|GetWorldLocation (Variables|/Game/Characters/BP_ThirdPersonCharacter_Base.BP_ThirdPersonCharacter_Base_C|GetCamera%20Prompt _player_reference)))) (Utilities|Time|GetWorldDeltaSeconds) 7.5) false false))
      (:else))))

(fn ConstructionScript)