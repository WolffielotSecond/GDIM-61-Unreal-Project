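; BP_EnemyController is the enemy AI controller that runs BT_Enemy and drives its chase, attack and stun Blackboard keys.
; Perception tracks Player-tagged actors and updates the enemy's state on sighting.
; Tick raises a sight timer toward the chase threshold, then counts it down when sight is lost, chasing until zero.
; Attack requires range and a full timer; PursuePlayer forces a chase, and Stuned flags a stun.
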(event OnTargetPerceptionUpdated(AIPerception)
  (params (Actor :type Actor%20Object%20Reference) (Stimulus :type AI%20Stimulus%20Structure))
  (bind _bsuccessfullysensed (Utilities|Struct|BreakAIStimulus Stimulus))
  (if (Actor|ActorHasTag Actor "Player")
    (Variables|Default|SetPlayer%20Actor Actor)
    (Variables|Default|SetIsSeenPlayer _bsuccessfullysensed)
    (if _bsuccessfullysensed
      (bind _asbp_enemy_base (Utilities|Casting|CastToBP_EnemyBase (Pawn|GetControlledPawn)))
      (Variables|/Game/Enemies/BP_EnemyBase.BP_EnemyBase_C|SetEnemy%20State _asbp_enemy_base "NewEnumerator1"))))

(event Custom|Stuned
  (AI|Components|Blackboard|SetValueasBool (Variables|Default|GetBlackboard) (Variables|Default|GetisStuned) true))

(event Custom|Pursue%20Player
  (bind _blackboard (Variables|Default|GetBlackboard))
  (Variables|Default|SetSeenTimer 5.0)
  (AI|Components|Blackboard|SetValueasBool _blackboard (Variables|Default|GetShouldChase) true)
  (AI|Components|Blackboard|SetValueasObject _blackboard (Variables|Default|GetChasePlayer) (Variables|Default|GetPlayer%20Actor)))

(event EventPossess
  (params (PossessedPawn :type Pawn%20Object%20Reference))
  (AI|RunBehaviorTree "/Game/Enemies/BT_Enemy.BT_Enemy"))

(event EventTick
  (params (DeltaSeconds :type Float%20%28single-precision%29))
  (bind _attackplayer (Variables|Default|GetAttackPlayer))
  (bind _blackboard (Variables|Default|GetBlackboard))
  (bind _blackboard_2 (Variables|Default|GetBlackboard))
  (Utilities|FlowControl|Sequence
    (:then_0
      (if (Variables|Default|GetIsSeenPlayer)
        (bind _output_get (Variables|Default|SetSeenTimer (Math|Float|Clamp(Float) (+ (Variables|Default|GetSeenTimer) DeltaSeconds) 0.0 (Variables|Default|GetChaseTimeNeeded))))
        (if (>= _output_get (Variables|Default|GetChaseTimeNeeded))
          (AI|Components|Blackboard|SetValueasBool _blackboard (Variables|Default|GetShouldChase) true :!label _label)
          (AI|Components|Blackboard|SetValueasObject _blackboard (Variables|Default|GetChasePlayer) (Variables|Default|GetPlayer%20Actor)))
        (else
          (bind _output_get_2 (Variables|Default|SetSeenTimer (Math|Float|Clamp(Float) (- (Variables|Default|GetSeenTimer) DeltaSeconds) 0.0 9999999.0)))
          (if (<= _output_get_2 0.0)
            (AI|Components|Blackboard|SetValueasBool (Variables|Default|GetBlackboard) (Variables|Default|GetShouldChase) false)
            (else
              (goto _label))))))
    (:then_1
      (if (and (< (Math|Vector|Distance(Vector) (Transformation|GetActorLocation (Game|Player|GetPlayerPawn 0)) (Transformation|GetActorLocation (Pawn|GetControlledPawn))) (Variables|Default|GetAttackRange)) (>= (Variables|Default|GetSeenTimer) (Variables|Default|GetChaseTimeNeeded)))
        (AI|Components|Blackboard|SetValueasBool _blackboard_2 _attackplayer true)
        (else
          (AI|Components|Blackboard|SetValueasBool _blackboard_2 _attackplayer false))))))

(fn ConstructionScript)