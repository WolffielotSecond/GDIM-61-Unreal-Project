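; BP_Dummy is a training-style enemy that repeatedly attacks and can be stunned by player parries or knife hits.
; Tick loops the attack montage, counts down stun time and shows a melee prompt when the player is near the stunned dummy.
; DamageDetection sphere-traces ahead for parries only, while melee triggers a recovery montage and target-lock events drive a prompt widget.
; Booleans drive behavior; ChangeState is an unused placeholder that prints debug text.
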(event Custom|Attack
  (Animation|Montage|PlayMontage (Variables|Character|GetMesh) "/Game/Characters/Mannequins/Anims/Attack/Dummy_Attack.Dummy_Attack"
    (:then
      (Variables|Default|SetIs%20attacking true))
    (:OnCompleted
      (Variables|Default|SetIs%20attacking false))
    (:OnInterrupted
      (Variables|Default|SetIs%20attacking false))))

(event EventBeginPlay
  (bind _aswb_auto_lock (Utilities|Casting|CastToWB_Auto_Lock (UserInterface|GetWidget (Variables|Default|GetTarget%20Lock%20Prompt))))
  (Variables|Default|SetAuto%20Lock%20Widget _aswb_auto_lock)
  (Rendering|SetVisibility (Variables|Default|GetTarget%20Lock%20Prompt) false false))

(event Collision|EventActorBeginOverlap
  (params (OtherActor :type Actor%20Object%20Reference)))

(event EventTick
  (params (DeltaSeconds :type Float%20%28single-precision%29))
  (Utilities|FlowControl|Sequence
    (:then_0
      (if (not (Variables|Default|GetIs%20attacking))
        (if (and (not (Variables|Default|GetStunned)) (not (Variables|Default|GetRecovering)))
          (CallFunction|Attack))))
    (:then_1
      (if (Variables|Default|GetStunned)
        (if (<= (Variables|Default|Gettimer) 0.0)
          (Variables|Default|SetStunned false))))
    (:then_2
      (if (> (Variables|Default|Gettimer) 0.0)
        (Variables|Default|Settimer (- (Variables|Default|Gettimer) (Utilities|Time|GetWorldDeltaSeconds)))))
    (:then_3
      (if (and (Variables|Default|GetStunned) (<= (Transformation|GetDistanceTo (Game|GetPlayerCharacter 0)) 2e+02))
        (Rendering|SetVisibility (Variables|Default|GetMelee%20Prompt) true false)
        (else
          (Rendering|SetVisibility (Variables|Default|GetMelee%20Prompt) false false))))))

(event EventDamageDetection
  (bind _returnvalue (Transformation|GetActorLocation))
  (bind _returnvalue_2 (Transformation|GetActorForwardVector))
  (bind _returnvalue_3 (* _returnvalue_2 1e+02))
  (bind _returnvalue_4 (+ _returnvalue _returnvalue_3))
  (bind (_outhit _returnvalue_5) (Collision|SphereTraceForObjects _returnvalue_4 _returnvalue_4 1e+02 (Utilities|Array|MakeArray "ObjectTypeQuery3") false 0 "None"))
  (if _returnvalue_5
    (if (Actor|ActorHasTag (.HitActor (Collision|BreakHitResult _outhit)) "Player")
      (bind _asbp_third_person_character_base (Utilities|Casting|CastToBP_ThirdPersonCharacter_Base (.HitActor (Collision|BreakHitResult _outhit))))
      (if (Variables|/Game/Characters/BP_ThirdPersonCharacter_Base.BP_ThirdPersonCharacter_Base_C|GetParry%20Window _asbp_third_person_character_base)
        (Default|OnSuccessfulParry _asbp_third_person_character_base self)
        (Animation|StopAnimMontage 0)
        (Variables|Default|Settimer 1e+03)
        (Variables|Default|SetStunned true)))))

(event EventOnBeingMeleed
  (Animation|Montage|PlayMontage (Variables|Character|GetMesh) "/Game/Characters/Mannequins/Anims/Attack/RecoveringFromStun_Montage.RecoveringFromStun_Montage"
    (:then
      (Variables|Default|SetStunned false)
      (Variables|Default|SetRecovering true))
    (:OnCompleted
      (Variables|Default|SetRecovering false))
    (:OnInterrupted
      (Variables|Default|SetRecovering false))))

(event EventOnTargetLock
  (Default|PlayonTargetLockedAnimation (Variables|Default|GetAuto%20Lock%20Widget))
  (Rendering|SetVisibility (Variables|Default|GetTarget%20Lock%20Prompt) true false))

(event EventOnTargetUnlock
  (Rendering|SetVisibility (Variables|Default|GetTarget%20Lock%20Prompt) false false))

(event EventOnPlayerKnifeHit
  (Variables|Default|Settimer 3.0)
  (Variables|Default|SetStunned true)
  (Animation|StopAnimMontage 0)
  (Default|SplatterBlood (Variables|Default|GetBPC_Blood_Splatter)))

(fn ConstructionScript)

(fn ChangeState
  (params (New%20State :type E_Enemy_State%20Enum :default "NewEnumerator0"))
  (if (not (Utilities|Enum|Equal(Enum) New%20State (Variables|Default|GetCurrent%20State)))
    ;[0.15 0.15 0.15 0.5] Exit
    (switch Utilities|FlowControl|Switch|SwitchonE_Enemy_State (Variables|Default|GetCurrent%20State)
      (:NewEnumerator3
        _)
      (:NewEnumerator4
        _)
      (:NewEnumerator5
        _))
    (Development|PrintString "Hello")
    (bind _output_get (Variables|Default|SetCurrent%20State New%20State))
    (switch Utilities|FlowControl|Switch|SwitchonE_Enemy_State _output_get
      (:NewEnumerator3
        _)
      (:NewEnumerator4
        _)
      (:NewEnumerator5
        _))
    (Development|PrintString "Hello")))

(fn GetIsStunned
  (return (Variables|Default|GetStunned)))