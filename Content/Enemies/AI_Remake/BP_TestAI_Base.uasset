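; BP_TestAI_Base is a base test enemy that can attack the player and shows a prompt when target-locked.
; BeginPlay caches the WB_Auto_Lock widget from TargetLockPrompt and hides it; lock and unlock events toggle it, with an animation on lock.
; AttackPlayer plays the Dummy_Attack montage and calls CallFinishAttackAnim on completion or interruption.
; GetIsStunned always returns false, and the ChasePlayer call is unconnected.
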(event Custom|Attack%20Player
  (Animation|Montage|PlayMontage (Variables|Character|GetMesh) "/Game/Characters/Mannequins/Anims/Attack/Dummy_Attack.Dummy_Attack"
    (:OnCompleted
      _)
    (:OnInterrupted
      _))
  (Default|CallFinishAttackAnim))

(event EventBeginPlay
  (Utilities|FlowControl|Sequence
    (:then_0
      (bind _aswb_auto_lock (Utilities|Casting|CastToWB_Auto_Lock (UserInterface|GetWidget (Variables|Default|GetTarget%20Lock%20Prompt))))
      (Variables|Default|SetAuto%20Lock%20Widget _aswb_auto_lock)
      (Rendering|SetVisibility (Variables|Default|GetTarget%20Lock%20Prompt) false false))))

(event Collision|EventActorBeginOverlap
  (params (OtherActor :type Actor%20Object%20Reference)))

(event EventTick
  (params (DeltaSeconds :type Float%20%28single-precision%29)))

(event EventOnTargetLock
  (Default|PlayonTargetLockedAnimation (Variables|Default|GetAuto%20Lock%20Widget))
  (Rendering|SetVisibility (Variables|Default|GetTarget%20Lock%20Prompt) true false))

(event EventOnTargetUnlock
  (Rendering|SetVisibility (Variables|Default|GetTarget%20Lock%20Prompt) false false))

(fn ConstructionScript)

(fn GetIsStunned
  (return false))