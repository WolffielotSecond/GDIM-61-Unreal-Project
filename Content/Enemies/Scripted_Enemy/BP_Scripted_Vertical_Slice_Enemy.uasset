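; Scripted vertical-slice enemy that drives a chase set piece and then a combat tutorial against the player.
; Event-driven beats run camera cutscenes with shakes, break a wall and vault object, teleport the enemy at the safe room, save, and reset on Reload.
; Tick velocity-steers it at the player; its lunge either triggers death or, if the player has a knife, a paused parry tutorial leading to stun, melee and knife-hit damage until death.
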(event Custom|Start%20Pursuing
  (Pawn|Components|CharacterMovement|SetMovementMode (Variables|Character|GetCharacterMovement) "MOVE_Walking" 0)
  (Character|LaunchCharacter (+ (* (Math|Vector|GetForwardVector (Math|Rotator|MakeRotator 0.0 0.0 (.yaw (Math|Rotator|FindLookatRotation (Transformation|GetActorLocation) (Transformation|GetActorLocation (Game|GetPlayerCharacter 0)))))) 3e+02) "0.000000,0.000000,200.000000") false false)
  (Variables|Default|SetLaunched true)
  (Collision|SetCollisionEnabled (Variables|/Game/Enemies/Scripted_Enemy/BP_Scripted_enemy_event_trigger.BP_Scripted_enemy_event_trigger_C|GetBox (Variables|Default|GetStart%20Pursuing%20Block)) "NoCollision")
  (Development|PrintString "Launch"))

(event Custom|Destroy%20Wall
  (bind _returnvalue (Niagara|SpawnSystematLocation "/Game/FX/NS_Fx_HookRope.NS_Fx_HookRope" (Transformation|GetWorldLocation (Variables|/Game/Blueprints/Breakable_wall/BP_Breakable_Wall.BP_Breakable_Wall_C|GetHit%20point (Variables|Default|GetDestructable%20Wall)))))
  (Variables|Default|SetSystem _returnvalue)
  (Variables|Default|SetSet%20spawn%20lazer true)
  (Niagara|SetNiagaraVariable(Vector3) _returnvalue "End" (Transformation|GetWorldLocation (Variables|Default|GetEye%20Start)))
  (Default|Break (Variables|Default|GetDestructable%20Wall))
  (Collision|SetCollisionEnabled (Variables|/Game/Enemies/Scripted_Enemy/BP_Scripted_enemy_event_trigger.BP_Scripted_enemy_event_trigger_C|GetBox (Variables|Default|GetBreak%20Wall%20Trigger)) "NoCollision"))

(event Custom|Attack
  (Variables|Default|SetAttacking true)
  (Variables|Default|SetShould%20Pursue%20Player false)
  (Character|LaunchCharacter (+ (* (Math|Vector|GetForwardVector (Math|Rotator|MakeRotator 0.0 0.0 (.yaw (Math|Rotator|FindLookatRotation (Transformation|GetActorLocation) (Transformation|GetActorLocation (Game|GetPlayerCharacter 0)))))) 3e+02) "0.000000,0.000000,300.000000") false false)
  (if (Variables|/Game/Characters/BP_ThirdPersonCharacter_Base.BP_ThirdPersonCharacter_Base_C|GetHas%20Knife (Variables|Default|GetPlayer))
    (CallFunction|EnterParryTutorial)
    (else
      (Class|BPIGamecontroller|ScriptEnemyDeath(Message) (Game|GetPlayerController 0)))))

(event Custom|Break%20Vault%20Object
  (bind _vault_object (Variables|Default|GetVault%20Object))
  (Rendering|SetVisibility (Variables|/Script/Engine.StaticMeshActor|GetStaticMeshComponent _vault_object) false false)
  (Collision|SetCollisionEnabled (Variables|/Script/Engine.StaticMeshActor|GetStaticMeshComponent _vault_object) "NoCollision")
  (Collision|SetCollisionEnabled (Variables|/Game/Enemies/Scripted_Enemy/BP_Scripted_enemy_event_trigger.BP_Scripted_enemy_event_trigger_C|GetBox (Variables|Default|GetBreak%20Vault%20Object%20Trigger)) "NoCollision"))

(event Custom|Player%20Entered%20Safe%20Room
  (Actor|DestroyActor (Variables|Default|GetDestructable%20Wall))
  (Actor|DestroyActor (Variables|Default|GetInitial%20Camera))
  (Actor|DestroyActor (Variables|Default|GetStart%20Pursuing%20Block))
  (Actor|DestroyActor (Variables|Default|GetBreak%20Wall%20Trigger))
  (Actor|DestroyActor (Variables|Default|GetBreak%20Vault%20Object%20Trigger))
  (Actor|DestroyActor (Variables|Default|GetVault%20Object))
  (Class|BPIGamecontroller|SaveGame(Message) (Game|GetPlayerController 0))
  (Variables|Default|SetShould%20Pursue%20Player false)
  (Transformation|SetActorLocation (Variables|Default|GetSaferoom%20out%20location) false false)
  (Variables|/Game/Characters/BP_ThirdPersonCharacter_Base.BP_ThirdPersonCharacter_Base_C|Sethas%20entered%20safe%20room (Variables|Default|GetPlayer) true))

(event Custom|Player%20exit%20safe%20room
  (Input|DisableInput (Game|GetPlayerCharacter 0) (Game|GetPlayerController 0))
  (Game|Player|SetViewTargetwithBlend (Game|GetPlayerController 0) (Variables|Default|Getbattle%20tutorial%20camera%20ref) 1.5 "VTBlend_Linear" 0.0 false)
  (Utilities|FlowControl|Delay 2.0)
  (CallFunction|PrepareforTutorial))

(event Custom|Prepare%20for%20tutorial
  (Variables|/Game/Characters/BP_ThirdPersonCharacter_Base.BP_ThirdPersonCharacter_Base_C|Setentered%20parry%20tutorial (Variables|Default|GetPlayer) true)
  (Variables|/Game/Characters/BP_ThirdPersonCharacter_Base.BP_ThirdPersonCharacter_Base_C|Setentered%20battle%20tutorial (Variables|Default|GetPlayer) true)
  (Camera|PlayWorldCameraShake "/Game/Blueprints/Camera_Shakes/BP_Enemy_roar_Shake.BP_Enemy_roar_Shake_C" (Transformation|GetWorldLocation (Variables|/Script/Engine.CameraActor|GetCameraComponent (Variables|Default|Getbattle%20tutorial%20camera%20ref))) 0.0 5e+02)
  (Utilities|FlowControl|Delay 2.0)
  (Utilities|FlowControl|Delay 0.5)
  (Game|Player|SetViewTargetwithBlend (Game|GetPlayerController 0) (Variables|/Game/Characters/BP_ThirdPersonCharacter_Base.BP_ThirdPersonCharacter_Base_C|GetCamera%20Actor%20Reference (Variables|Default|GetPlayer)) 0.5 "VTBlend_Linear" 0.0 false)
  (Input|EnableInput (Game|GetPlayerCharacter 0) (Game|GetPlayerController 0))
  (Variables|Default|SetShould%20Pursue%20Player true))

(event Custom|Enter%20Parry%20Tutorial
  (Variables|/Game/Characters/BP_ThirdPersonCharacter_Base.BP_ThirdPersonCharacter_Base_C|Setentered%20parry%20tutorial (Variables|Default|GetPlayer) false)
  (Class|BPIPlayerInterface|PlayTutorialMessage(Message) (Game|GetPlayerCharacter 0) "Parry with Right Mouse Button" false 0.0 "Parry with RB" true "Parry")
  (Variables|/Game/Characters/BP_ThirdPersonCharacter_Base.BP_ThirdPersonCharacter_Base_C|SetCurrent%20Downed%20Enemy (Variables|Default|GetPlayer) self)
  (Game|SetGamePaused true)
  (Development|PrintString "Entered Tutorial"))

(event Custom|Die
  (bind _player (Variables|Default|GetPlayer))
  (bind _enemies (Variables|/Game/Characters/BP_ThirdPersonCharacter_Base.BP_ThirdPersonCharacter_Base_C|GetEnemies _player))
  (bind _player_exit_room_trigger (Variables|Default|GetPlayer%20Exit%20Room%20Trigger)
    (:then
      (Actor|DestroyActor _player_exit_room_trigger))
    (:else
      _))
  (Actor|DestroyActor (Variables|Default|Getbattle%20tutorial%20camera%20ref))
  (Class|BPIGamecontroller|SaveGame(Message) (Game|GetPlayerController 0))
  (Utilities|Array|RemoveIndex _enemies (Utilities|Array|FindItem _enemies self))
  (Actor|DestroyActor))

(event EventBeginPlay
  (Collision|SetCollisionEnabled (Variables|/Game/Blueprints/BP_Camera_MoveBackBox.BP_Camera_MoveBackBox_C|GetDetection%20Box (Variables|Default|GetCamera%20Move%20Back%20Box)) "NoCollision")
  (bind _asbp_third_person_character_base (Utilities|Casting|CastToBP_ThirdPersonCharacter_Base (Game|GetPlayerCharacter 0)))
  (Variables|Default|SetPlayer _asbp_third_person_character_base)
  (Variables|Default|SetDefault%20Location (Transformation|GetActorLocation))
  (Variables|Default|SetDefault%20Rotation (Transformation|GetActorRotation)))

(event Collision|EventActorBeginOverlap
  (params (OtherActor :type Actor%20Object%20Reference)))

(event EventOnPlayerKnifeHit
  (Default|SplatterBlood (Variables|Default|GetBPC_Blood_Splatter))
  (Variables|Default|SetHealth (- (Variables|Default|GetHealth) 1e+01))
  (if (<= (Variables|Default|GetHealth) 0.0)
    (CallFunction|Die)
    (else
      (Character|LaunchCharacter (+ (* (Math|Vector|GetForwardVector (Math|Rotator|MakeRotator 0.0 0.0 (.yaw (Math|Rotator|FindLookatRotation (Transformation|GetActorLocation (Game|GetPlayerCharacter 0)) (Transformation|GetActorLocation))))) 1e+02) "0.000000,0.000000,100.000000") false false))))

(event EventActivateEscapeSequence
  (Input|DisableInput (Game|GetPlayerCharacter 0) (Game|GetPlayerController 0))
  (Camera|PlayWorldCameraShake "/Game/Blueprints/Camera_Shakes/BP_Knife_Hit_Shake.BP_Knife_Hit_Shake_C" (Transformation|GetWorldLocation (Variables|/Game/Blueprints/BP_Camera.BP_Camera_C|GetCamera (Variables|/Game/Characters/BP_ThirdPersonCharacter_Base.BP_ThirdPersonCharacter_Base_C|GetCamera%20Actor%20Reference (Variables|Default|GetPlayer)))) 0.0 5e+02)
  (Utilities|FlowControl|Delay 1.0)
  (Game|Player|SetViewTargetwithBlend (Game|GetPlayerController 0) (Variables|Default|GetInitial%20Camera) 1.5 "VTBlend_Linear" 0.0 false)
  (Utilities|FlowControl|Delay 2.0)
  (Camera|PlayWorldCameraShake "/Game/Blueprints/Camera_Shakes/BP_Test_CameraShake.BP_Test_CameraShake_C" (Transformation|GetWorldLocation (Variables|/Script/Engine.CameraActor|GetCameraComponent (Variables|Default|GetInitial%20Camera))) 0.0 5e+02)
  (Actor|DestroyActor (Variables|Default|GetInitial%20Move%20Back%20Box))
  (Actor|DestroyActor (Variables|Default|GetReveal%20Breakable%20Wall))
  (Utilities|FlowControl|Delay 1.0)
  (Camera|PlayWorldCameraShake "/Game/Blueprints/Camera_Shakes/BP_Enemy_roar_Shake.BP_Enemy_roar_Shake_C" (Transformation|GetWorldLocation (Variables|/Script/Engine.CameraActor|GetCameraComponent (Variables|Default|GetInitial%20Camera))) 0.0 5e+02)
  (Utilities|FlowControl|Delay 2.0)
  (Collision|SetCollisionEnabled (Variables|/Game/Blueprints/BP_Camera_MoveBackBox.BP_Camera_MoveBackBox_C|GetDetection%20Box (Variables|Default|GetCamera%20Move%20Back%20Box)) "QueryOnly")
  (bind _asbp_third_person_character_base (Utilities|Casting|CastToBP_ThirdPersonCharacter_Base (Game|GetPlayerCharacter 0)))
  (Input|EnableInput (Game|GetPlayerCharacter 0) (Game|GetPlayerController 0))
  (Game|Player|SetViewTargetwithBlend (Game|GetPlayerController 0) (Variables|/Game/Characters/BP_ThirdPersonCharacter_Base.BP_ThirdPersonCharacter_Base_C|GetCamera%20Actor%20Reference _asbp_third_person_character_base) 1.0 "VTBlend_Linear" 0.0 false)
  (Utilities|FlowControl|Delay 1.0)
  (Class|BPIPlayerInterface|PlayTutorialMessage(Message) (Game|GetPlayerCharacter 0) "Sprint With L Shift" false 0.0 "Sprint By Holding LS" false "None"))

(event EventTick
  (params (DeltaSeconds :type Float%20%28single-precision%29))
  (Utilities|FlowControl|Sequence
    (:then_0
      (if (Variables|Default|GetShould%20Pursue%20Player)
        (Variables|/Script/Engine.MovementComponent|SetVelocity (Variables|Character|GetCharacterMovement) (* (Math|Vector|GetForwardVector (Math|Rotator|MakeRotator 0.0 0.0 (.yaw (Math|Rotator|FindLookatRotation (Transformation|GetActorLocation) (Transformation|GetActorLocation (Game|GetPlayerCharacter 0)))))) 8.5e+02))
        (Transformation|SetActorRotation (Math|Rotator|MakeRotator 0.0 0.0 (.yaw (Math|Rotator|FindLookatRotation (Transformation|GetActorLocation) (Transformation|GetActorLocation (Game|GetPlayerCharacter 0))))))
        (if (<= (Transformation|GetDistanceTo (Game|GetPlayerCharacter 0)) 2e+02)
          (CallFunction|Attack))))
    (:then_1
      (if (Variables|Default|GetSet%20spawn%20lazer)
        (bind _system (Variables|Default|GetSystem)
          (:then
            (Niagara|SetNiagaraVariable(Vector3) _system "End" (Transformation|GetWorldLocation (Variables|Default|GetEye%20Start)))
            (Utilities|FlowControl|DoOnce false :!label _label
              (:Completed
                (Utilities|FlowControl|Delay (Variables|Default|GetLazer%20Duration))
                (Variables|Default|SetSet%20spawn%20lazer false))))
          (:else))
        (else
          (goto _label Reset))))
    (:then_2
      (if (Variables|Default|Getshould%20turn%20mesh)
        (Transformation|SetActorRotation (Math|Interpolation|RInterpTo (Transformation|GetActorRotation) (Math|Rotator|MakeRotator 0.0 0.0 (.yaw (Math|Rotator|FindLookatRotation (Transformation|GetActorLocation) (Transformation|GetActorLocation (Game|GetPlayerCharacter 0))))) (Utilities|Time|GetWorldDeltaSeconds) 2.0))
        (if (Utilities|Operators|EqualEqual (Transformation|GetActorRotation) (Math|Rotator|MakeRotator 0.0 0.0 (.yaw (Math|Rotator|FindLookatRotation (Transformation|GetActorLocation) (Transformation|GetActorLocation (Game|GetPlayerCharacter 0))))) 0.08)
          (Variables|Default|Setshould%20turn%20mesh false)
          (CallFunction|PrepareforTutorial))))
    (:then_3
      (if (and (Variables|Default|Getis%20stunned) (<= (Transformation|GetDistanceTo (Game|GetPlayerCharacter 0)) 2e+02))
        (Rendering|SetVisibility (Variables|Default|GetWidget) true false)
        (else
          (Rendering|SetVisibility (Variables|Default|GetWidget) false false))))))

(event EventOnLanded
  (params (Hit :type Hit%20Result%20Structure%20%28by%20ref%29))
  (Utilities|FlowControl|Sequence
    (:then_0
      (if (Variables|Default|GetLaunched)
        (Variables|Default|SetLaunched false)
        (Variables|Default|SetShould%20Pursue%20Player true)))
    (:then_1
      (if (Variables|Default|GetAttacking)
        (Variables|Default|SetAttacking false)))))

(event EventReload
  (bind _destructable_wall (Variables|Default|GetDestructable%20Wall))
  (bind _vault_object (Variables|Default|GetVault%20Object))
  (bind _cube (Variables|/Game/Blueprints/Breakable_wall/BP_Breakable_Wall.BP_Breakable_Wall_C|GetCube _destructable_wall))
  (Variables|Default|SetAttacking false)
  (Variables|Default|SetShould%20Pursue%20Player false)
  (Rendering|SetVisibility _cube true true)
  (Collision|SetCollisionEnabled _cube "QueryAndPhysics")
  (Rendering|SetVisibility (Variables|/Script/Engine.StaticMeshActor|GetStaticMeshComponent _vault_object) true false)
  (Collision|SetCollisionEnabled (Variables|/Script/Engine.StaticMeshActor|GetStaticMeshComponent _vault_object) "QueryAndPhysics")
  (Collision|SetCollisionEnabled (Variables|/Game/Enemies/Scripted_Enemy/BP_Scripted_enemy_event_trigger.BP_Scripted_enemy_event_trigger_C|GetBox (Variables|Default|GetStart%20Pursuing%20Block)) "QueryOnly")
  (Collision|SetCollisionEnabled (Variables|/Game/Enemies/Scripted_Enemy/BP_Scripted_enemy_event_trigger.BP_Scripted_enemy_event_trigger_C|GetBox (Variables|Default|GetBreak%20Wall%20Trigger)) "QueryOnly")
  (Collision|SetCollisionEnabled (Variables|/Game/Enemies/Scripted_Enemy/BP_Scripted_enemy_event_trigger.BP_Scripted_enemy_event_trigger_C|GetBox (Variables|Default|GetBreak%20Vault%20Object%20Trigger)) "QueryOnly")
  (Collision|SetCollisionEnabled (Variables|/Game/Enemies/Scripted_Enemy/BP_Scripted_enemy_event_trigger.BP_Scripted_enemy_event_trigger_C|GetBox (Variables|Default|GetPlayer%20Enter%20Room%20Trigger)) "QueryOnly")
  (Collision|SetCollisionEnabled (Variables|/Game/Enemies/Scripted_Enemy/BP_Scripted_enemy_event_trigger.BP_Scripted_enemy_event_trigger_C|GetBox (Variables|Default|GetPlayer%20Exit%20Room%20Trigger)) "QueryOnly")
  (Transformation|SetActorLocationAndRotation (Variables|Default|GetDefault%20Location) (Variables|Default|GetDefault%20Rotation)))

(event EventOnParried
  (Utilities|FlowControl|Delay 0.1)
  (Default|OnSuccessfulParry (Variables|Default|GetPlayer) self)
  (Variables|Default|Setis%20stunned true)
  (Variables|Default|SetShould%20Pursue%20Player false)
  (Variables|Default|SetAttacking false)
  (Variables|/Script/Engine.MovementComponent|SetVelocity (Variables|Character|GetCharacterMovement) "0, 0, 0")
  (Character|LaunchCharacter (+ (* (Math|Vector|GetForwardVector (Math|Rotator|MakeRotator 0.0 0.0 (.yaw (Math|Rotator|FindLookatRotation (Transformation|GetActorLocation (Game|GetPlayerCharacter 0)) (Transformation|GetActorLocation))))) 3e+02) "0.000000,0.000000,300.000000") false false)
  (Class|BPIPlayerInterface|PlayTutorialMessage(Message) (Game|GetPlayerCharacter 0) "Melee Stunned Enemy with F" false 0.0 "Melee Stunned Enemy with Y" false "None"))

(event EventOnBeingMeleed
  (Variables|Default|Setis%20stunned false)
  (Variables|/Game/Characters/BP_ThirdPersonCharacter_Base.BP_ThirdPersonCharacter_Base_C|Setentered%20battle%20tutorial (Variables|Default|GetPlayer) false)
  (Class|BPIPlayerInterface|PlayTutorialMessage(Message) (Game|GetPlayerCharacter 0) "Attack the Enemy with LMB" false 0.0 "Attack the Enemy with X" false "None")
  (Character|LaunchCharacter (+ (* (Math|Vector|GetForwardVector (Math|Rotator|MakeRotator 0.0 0.0 (.yaw (Math|Rotator|FindLookatRotation (Transformation|GetActorLocation (Game|GetPlayerCharacter 0)) (Transformation|GetActorLocation))))) 3e+02) "0.000000,0.000000,300.000000") false false))

(fn ConstructionScript)

(fn GetIsStunned
  (return (Variables|Default|Getis%20stunned)))