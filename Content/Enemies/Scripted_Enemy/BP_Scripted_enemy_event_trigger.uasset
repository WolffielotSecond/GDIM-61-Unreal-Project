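; BP_Scripted_enemy_event_trigger is a box trigger that drives scripted moments for a referenced enemy in an escape or chase sequence.
; On overlap it switches on ColliderType to start pursuit, destroy a wall, break a vault object, or signal the player entering or exiting a safe room.
; Each case checks a Player or Enemy tag, some also check player escape-sequence or knife state, and safe-room triggers destroy themselves after firing.
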(event OnComponentBeginOverlap(Box)
  (params (OverlappedComponent :type Primitive%20Component%20Object%20Reference) (OtherActor :type Actor%20Object%20Reference) (OtherComp :type Primitive%20Component%20Object%20Reference) (OtherBodyIndex :type Integer) (bFromSweep :type Boolean) (SweepResult :type Hit%20Result%20Structure%20%28by%20ref%29))
  (bind _returnvalue (Actor|ActorHasTag OtherActor "Player"))
  (switch Utilities|FlowControl|Switch|SwitchonE_Scripted_Enemy_Event_TriggerType (Variables|Default|GetCollider%20Type)
    (:NewEnumerator0
      (if _returnvalue
        (if (Variables|/Game/Characters/BP_ThirdPersonCharacter_Base.BP_ThirdPersonCharacter_Base_C|GetEscape%20Sequence%20VS%20done (Variables|Default|GetPlayer))
          (Default|StartPursuing (Variables|Default|GetEnemy%20Reference)))))
    (:NewEnumerator1
      (if _returnvalue
        (if (Variables|/Game/Characters/BP_ThirdPersonCharacter_Base.BP_ThirdPersonCharacter_Base_C|GetEscape%20Sequence%20VS%20done (Variables|Default|GetPlayer))
          (Default|DestroyWall (Variables|Default|GetEnemy%20Reference)))))
    (:NewEnumerator2
      (if (Actor|ActorHasTag OtherActor "Enemy")
        (Default|BreakVaultObject (Variables|Default|GetEnemy%20Reference))))
    (:NewEnumerator3
      (if _returnvalue
        (Default|PlayerEnteredSafeRoom (Variables|Default|GetEnemy%20Reference))
        (Actor|DestroyActor)))
    (:NewEnumerator4
      (if _returnvalue
        (if (Variables|/Game/Characters/BP_ThirdPersonCharacter_Base.BP_ThirdPersonCharacter_Base_C|GetHas%20Knife (Variables|Default|GetPlayer))
          (Default|PlayerExitSafeRoom (Variables|Default|GetEnemy%20Reference))
          (Actor|DestroyActor))))))

(event EventBeginPlay
  (bind _asbp_third_person_character_base (Utilities|Casting|CastToBP_ThirdPersonCharacter_Base (Game|GetPlayerCharacter 0)))
  (Variables|Default|SetPlayer _asbp_third_person_character_base))

(fn ConstructionScript)