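; Base enemy character for melee combat, with lock-on widget, knockback, stun and death.
; While airborne in its attack state, Tick sphere-traces ahead for one hit on the player, who takes damage or parries to stun it through BP_EnemyController.
; Knife hits drain health and poise in BPCEntityStats.
; When stunned, it shows a melee prompt to a nearby player, and that melee launches it away with extra health loss.
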(event Custom|UpdateWalkSpeed
  (params (NewSpeed :type Float%20%28double-precision%29))
  (Variables|/Script/Engine.CharacterMovementComponent|SetMaxWalkSpeed (Variables|Character|GetCharacterMovement) NewSpeed))

(event Custom|Enemy%20Stunned
  (bind _asbp_enemy_controller (Utilities|Casting|CastToBP_EnemyController (Pawn|GetController)))
  (Default|Stuned _asbp_enemy_controller))

(event EventOnBeingMeleed
  (bind _returnvalue (Game|Player|GetPlayerPawn 0))
  (bind _self self)
  (bind _dashspeed (Variables|Default|GetDashSpeed))
  (bind _returnvalue_2 (Transformation|GetActorLocation _self))
  (bind _returnvalue_3 (Transformation|GetActorLocation _returnvalue))
  (bind _returnvalue_4 (- _returnvalue_2 _returnvalue_3))
  (bind _returnvalue_5 (Math|Vector|Normalize _returnvalue_4))
  ;[0.15 0.15 0.15 0.5] 在眩晕状态下被玩家体术攻击后触发
  (Character|LaunchCharacter (Math|Vector|MakeVector (* (.x _returnvalue_5) _dashspeed) (* (.y _returnvalue_5) _dashspeed) (Variables|Default|GetJumpStrength)) false false)
  (Variables|Default|SetEnemy%20State "NewEnumerator5")
  (Default|扣血 (Variables|Default|GetBPC_Entity_Stats) 3e+01))

(event EventDamageDetection
  ;[0.15 0.15 0.15 0.5] 敌人攻击判定（Trace然后打到玩家身上apply damage之类的
)

(event EventTick
  (params (DeltaSeconds :type Float%20%28single-precision%29))
  (bind _returnvalue (Transformation|GetActorLocation))
  (bind _returnvalue_2 (Transformation|GetActorForwardVector))
  (bind _returnvalue_3 (* _returnvalue_2 1e+02))
  (bind _returnvalue_4 (+ _returnvalue _returnvalue_3))
  (Utilities|FlowControl|Sequence
    (:then_0
      (if (and (Utilities|Enum|Equal(Enum) (Variables|Default|GetEnemy%20State) "NewEnumerator4") (<= (Transformation|GetDistanceTo (Game|GetPlayerCharacter 0)) 2e+02))
        (Rendering|SetVisibility (Variables|Default|GetMelee%20Prompt) true false)
        (else
          (Rendering|SetVisibility (Variables|Default|GetMelee%20Prompt) false false))))
    (:then_1
      (if (and (Utilities|Enum|Equal(Enum) (Variables|Default|GetEnemy%20State) "NewEnumerator3") (not (Variables|Default|GetAttacked)))
        (bind (_outhit _returnvalue_5) (Collision|SphereTraceForObjects _returnvalue_4 _returnvalue_4 1e+02 (Utilities|Array|MakeArray "ObjectTypeQuery3") false 0 "ForOneFrame"))
        (if _returnvalue_5
          (if (Actor|ActorHasTag (.HitActor (Collision|BreakHitResult _outhit)) "Player")
            (bind _asbp_third_person_character_base (Utilities|Casting|CastToBP_ThirdPersonCharacter_Base (.HitActor (Collision|BreakHitResult _outhit))))
            (Variables|Default|SetAttacked true)
            (if (Variables|/Game/Characters/BP_ThirdPersonCharacter_Base.BP_ThirdPersonCharacter_Base_C|GetParry%20Window _asbp_third_person_character_base)
              (Default|OnSuccessfulParry _asbp_third_person_character_base self)
              (bind _asbp_enemy_controller (Utilities|Casting|CastToBP_EnemyController (Pawn|GetController)))
              (Default|Stuned _asbp_enemy_controller)
              (else
                (Development|PrintString "Successful Hit")
                (Class|BPIPlayerInterface|DealDamage(Message) (Game|GetPlayerCharacter 0) 1e+01)))))))
    (:then_2
      (if (and (not (AI|Components|NavMovement|IsFalling (Variables|Character|GetCharacterMovement))) (Utilities|Enum|Equal(Enum) (Variables|Default|GetEnemy%20State) "NewEnumerator3"))
        (Variables|Default|SetEnemy%20State "NewEnumerator5")))))

(event EventOnTargetUnlock
  (Rendering|SetVisibility (Variables|Default|GetTarget%20Lock%20Widget) false false))

(event EventOnTargetLock
  (Default|PlayonTargetLockedAnimation (Variables|Default|GetAuto%20Lock%20Widget))
  (Rendering|SetVisibility (Variables|Default|GetTarget%20Lock%20Widget) true false))

(event EventBeginPlay
  (bind _aswb_auto_lock (Utilities|Casting|CastToWB_Auto_Lock (UserInterface|GetWidget (Variables|Default|GetTarget%20Lock%20Widget))))
  (Variables|Default|SetAuto%20Lock%20Widget _aswb_auto_lock)
  (Rendering|SetVisibility (Variables|Default|GetTarget%20Lock%20Widget) false false))

(event Custom|Die
  (Actor|DestroyActor))

(event Custom|受击击退
  (bind _returnvalue (Game|Player|GetPlayerPawn 0))
  (bind _self self)
  (bind _被普攻dashspeed (Variables|Default|Get被普攻DashSpeed))
  (bind _returnvalue_2 (Transformation|GetActorLocation _self))
  (bind _returnvalue_3 (Transformation|GetActorLocation _returnvalue))
  (bind _returnvalue_4 (- _returnvalue_2 _returnvalue_3))
  (bind _returnvalue_5 (Math|Vector|Normalize _returnvalue_4))
  (Character|LaunchCharacter (Math|Vector|MakeVector (* (.x _returnvalue_5) _被普攻dashspeed) (* (.y _returnvalue_5) _被普攻dashspeed) (Variables|Default|Get被普攻JumpStrength)) false false))

(event EventOnPlayerKnifeHit
  (Default|扣韧 (Variables|Default|GetBPC_Entity_Stats) 4e+01)
  (Default|扣血 (Variables|Default|GetBPC_Entity_Stats) 1e+01))

(fn ConstructionScript)

(fn GetIsStunned
  (return (Utilities|Enum|Equal(Enum) (Variables|Default|GetEnemy%20State) "NewEnumerator4")))