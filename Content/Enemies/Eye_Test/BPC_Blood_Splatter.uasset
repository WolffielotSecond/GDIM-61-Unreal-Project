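; Actor component that spawns a blood splatter Niagara effect for its owning enemy.
; The SplatterBlood event spawns NS_Blood_Splatter at the owner's location, pushed toward the player character by ForwardOffset along a look-at rotation and raised by HeightOffset.
; Only the spawn position accounts for the player's direction, as no rotation is passed to the effect.
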(event Custom|Splatter%20Blood
  (bind _returnvalue (Components|GetOwner))
  (bind _returnvalue_2 (Transformation|GetActorLocation _returnvalue))
  (Niagara|SpawnSystematLocation "/Game/FX/NS_Blood_Splatter.NS_Blood_Splatter" (+ (+ _returnvalue_2 (* (Math|Vector|GetForwardVector (Math|Rotator|FindLookatRotation _returnvalue_2 (Transformation|GetActorLocation (Game|GetPlayerCharacter 0)))) (Variables|Default|GetForward%20Offset))) (Math|Vector|MakeVector 0.0 0.0 (Variables|Default|GetHeight%20Offset)))))

(event EventBeginPlay)

(event EventTick
  (params (DeltaSeconds :type Float%20%28single-precision%29)))