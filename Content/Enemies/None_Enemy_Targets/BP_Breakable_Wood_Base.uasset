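; Base breakable wood target that the player can lock onto and destroy with knife hits.
; On BeginPlay it caches the auto-lock widget and hides the lock prompt, then target lock and unlock events show or hide it, with an animation on lock.
; Each knife hit deducts fixed damage from Health, and the actor is destroyed when Health runs out.
; It always reports itself as not stunned.
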(event Custom|Health%20Deduction
  (params (Damage :type Float%20%28double-precision%29))
  (Variables|Default|SetHealth (- (Variables|Default|GetHealth) Damage))
  (CallFunction|ShouldBreak))

(event Custom|Should%20Break
  (if (<= (Variables|Default|GetHealth) 0.0)
    (CallFunction|BreakWood)))

(event Custom|Break%20Wood
  (Actor|DestroyActor))

(event EventBeginPlay
  (bind _aswb_auto_lock (Utilities|Casting|CastToWB_Auto_Lock (UserInterface|GetWidget (Variables|Default|GetTarget%20Lock%20Prompt))))
  (Variables|Default|SetAuto%20Lock%20Widget _aswb_auto_lock)
  (Rendering|SetVisibility (Variables|Default|GetTarget%20Lock%20Prompt) false false))

(event EventOnTargetLock
  (Default|PlayonTargetLockedAnimation (Variables|Default|GetAuto%20Lock%20Widget))
  (Rendering|SetVisibility (Variables|Default|GetTarget%20Lock%20Prompt) true false))

(event EventOnTargetUnlock
  (Rendering|SetVisibility (Variables|Default|GetTarget%20Lock%20Prompt) false false))

(event EventOnPlayerKnifeHit
  (CallFunction|HealthDeduction 1e+01))

(fn ConstructionScript)

(fn GetIsStunned
  (return false))