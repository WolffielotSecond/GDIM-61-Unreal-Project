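; Box volume actor for boss enemies that marks out a flying area and supplies random positions inside it.
; GetRandomPoint picks a random offset within the Box component's scaled extent on each axis and adds the box's world location.
; The offset ignores box rotation, so points fall in a world-axis-aligned region.
; The event graph and construction script hold no logic.
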(event EventBeginPlay)

(event Collision|EventActorBeginOverlap
  (params (OtherActor :type Actor%20Object%20Reference)))

(event EventTick
  (params (DeltaSeconds :type Float%20%28single-precision%29)))

(fn ConstructionScript)

(fn GetRandomPoint
  (bind _box (Variables|Default|GetBox))
  (bind _returnvalue (Components|Box|GetScaledBoxExtent _box))
  (return (+ (Math|Vector|MakeVector (Math|Random|RandomFloatinRange (* (.x _returnvalue) 1.0) (* (.x _returnvalue) -1.0)) (Math|Random|RandomFloatinRange (* (.y _returnvalue) 1.0) (* (.y _returnvalue) -1.0)) (Math|Random|RandomFloatinRange (* (.z _returnvalue) 1.0) (* (.z _returnvalue) -1.0))) (Transformation|GetWorldLocation _box))))