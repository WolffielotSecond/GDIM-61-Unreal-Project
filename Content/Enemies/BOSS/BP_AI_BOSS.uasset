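; Flying boss AI that roams random points in FlyingArea and, once active, attacks on a timer while no summoned minions remain.
; Its first three attacks run as laser, melee and summon, then random: telegraphed eye traces trailing the player, a chase into a spin, or Eye Monster spawns.
; BPCBossStats takes health and poise damage; stun drops the boss until recovery.
; Hit only resets its cooldown, leaving DamageDetection's parry-or-damage logic unwired.
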(event OnComponentBeginOverlap(Cube1)
  (params (OverlappedComponent :type Primitive%20Component%20Object%20Reference) (OtherActor :type Actor%20Object%20Reference) (OtherComp :type Primitive%20Component%20Object%20Reference) (OtherBodyIndex :type Integer) (bFromSweep :type Boolean) (SweepResult :type Hit%20Result%20Structure%20%28by%20ref%29))
  (if (== (Game|Player|GetPlayerPawn 0) OtherActor)
    (CallFunction|Hit 20 true)))

(event Custom|Lazer
  (Utilities|Shoot))

(event Custom|RandomMovement
  (if (not (Variables|Default|GetIsMeleeAttack))
    (Variables|Default|SetTarget%20Location (Default|GetRandomPoint (Variables|Default|GetFlyingArea)))))

(event Custom|Attack
  (if (not (> (Utilities|Array|Length (Variables|Default|GetSummonedEnemy)) 0))
    (if (Variables|Default|GetIsActive)
      (CallFunction|RandomAction))))

(event Custom|Active
  (Utilities|FlowControl|Delay 5.0)
  (Variables|Default|SetIsActive true)
  (CallFunction|RandomMovement)
  (Utilities|Time|SetTimerbyEvent (delegate Custom|Attack) 15.0 true)
  (Utilities|FlowControl|Delay 5.0)
  (CallFunction|RandomAction))

(event Custom|StartRotate
  (Variables|Default|SetIsRotating true)
  (Variables|Default|SetCurrentAngle 0.0))

(event EventBeginPlay
  (if (Variables|Default|GetIsActive)
    (CallFunction|Active)))

(event EventTick
  (params (DeltaSeconds :type Float%20%28single-precision%29))
  (bind _charactermovement (Variables|Character|GetCharacterMovement))
  (Utilities|FlowControl|Sequence
    (:then_0
      (if (Variables|Default|GetIsActive)
        (Variables|Default|SetDelta%20Seconds DeltaSeconds)
        (Utilities|FlowControl|Sequence
          (:then_0
            (CallFunction|BasicMovement))
          (:then_1
            (CallFunction|LazerChase))
          (:then_2
            (Variables|Default|SetHitTimer (- (Variables|Default|GetHitTimer) (Variables|Default|GetDelta%20Seconds))))
          (:then_3
            (CallFunction|MeleeCheck))
          (:then_4
            (if (> (Utilities|Array|Length (Variables|Default|GetSummonedEnemy)) 0)
              (CallFunction|EnemyCheck)))
          (:then_5
            (if (Variables|Default|GetIsRotating)
              (CallFunction|Rotate))))
        (elif (<= (.z (Transformation|GetActorLocation)) 295.0)
          (Variables|/Script/Engine.CharacterMovementComponent|SetGravityScale _charactermovement 0.0)
          (Variables|/Script/Engine.MovementComponent|SetVelocity _charactermovement "0, 0, 0"))))))

(event Custom|boss死亡
  ;[0.15 0.15 0.15 0.5] 添加boss死了之后的情节
  (Actor|DestroyActor))

(event Custom|boss%20被%20Stun
  ;[0.15 0.15 0.15 0.5] 后面添加被击晕后落地一系列操作
  (Variables|玩家交互|SetIs%20Stunned true)
  (Variables|/Script/Engine.CharacterMovementComponent|SetGravityScale (Variables|Character|GetCharacterMovement) 1.0)
  (Variables|Default|SetIsActive false))

(event Custom|BossRecover
  ;[0.15 0.15 0.15 0.5] 后面添加被踢恢复行动
  (Default|恢复韧性值 (Variables|Default|GetBPC_Boss_Stats))
  (Default|扣血 (Variables|Default|GetBPC_Boss_Stats) 75.0)
  (Variables|玩家交互|SetIs%20Stunned false)
  (Variables|Default|SetIsActive true))

(event EventOnPlayerKnifeHit
  (bind _bpc_boss_stats (Variables|Default|GetBPC_Boss_Stats))
  ;[0.15 0.15 0.15 0.5] 不用改
  (Default|扣血 _bpc_boss_stats 25.0)
  (Default|扣韧 _bpc_boss_stats 6e+01))

(event EventOnBeingMeleed
  ;[0.15 0.15 0.15 0.5] 后面添加被踢恢复行动
  (Default|恢复韧性值 (Variables|Default|GetBPC_Boss_Stats))
  (Default|扣血 (Variables|Default|GetBPC_Boss_Stats) 75.0)
  (Variables|玩家交互|SetIs%20Stunned false)
  (Variables|Default|SetIsActive true))

(event EventDamageDetection
  (params (Damage :type Float%20%28double-precision%29))
  ;[0.15 0.15 0.15 0.5] 在怪物普攻后调用这个function
  (bind _asbp_third_person_character_base (Utilities|Casting|CastToBP_ThirdPersonCharacter_Base (Game|GetPlayerCharacter 0)))
  (if (Variables|/Game/Characters/BP_ThirdPersonCharacter_Base.BP_ThirdPersonCharacter_Base_C|GetParry%20Window _asbp_third_person_character_base)
    (Default|OnSuccessfulParry _asbp_third_person_character_base self)
    (Default|扣韧 (Variables|Default|GetBPC_Boss_Stats) 1e+02)
    (else
      (Class|BPIPlayerInterface|DealDamage(Message) (Game|GetPlayerCharacter 0) Damage))))

(fn ConstructionScript)

(fn SetEyeMat
  (params (Material :type Material%20Object%20Reference))
  (Rendering|Material|SetMaterial (Variables|Default|GetEye1) 0 Material)
  (Rendering|Material|SetMaterial (Variables|Default|GetEye2) 0 Material))

(fn GetFlyingMoveDirection
  (params (TargetLocation :type Vector))
  (LocalVariables|SetToTarget (Math|Vector|Normalize (- TargetLocation (Transformation|GetWorldLocation (Variables|Default|GetPivot)))))
  (return (LocalVariables|GetToTarget)))

(fn ShootLazer
  (params (StartLocation :type Vector) (EndLocation :type Vector))
  (bind _outhit (Collision|SphereTraceByChannel StartLocation (* (Math|Vector|Normalize (- EndLocation StartLocation)) 9999999.0) 2e+01 "TraceTypeQuery1" false 0 "ForOneFrame"))
  (return (== (.HitActor (Collision|BreakHitResult _outhit)) (Game|Player|GetPlayerPawn 0))))

(fn RandomAction
  (if (Variables|Default|GetIsActive)
    (LocalVariables|SetRandomIndex (Math|Random|RandomIntegerinRange 1 3))
    (Variables|Default|SetCurrentRandomCount (+ (Variables|Default|GetCurrentRandomCount) 1))
    (if (== (Variables|Default|GetCurrentRandomCount) 1)
      (CallFunction|Lazer :!label _label)
      (elif (== (Variables|Default|GetCurrentRandomCount) 2)
        (CallFunction|MeleeAttack :!label _label_2)
        (else
          (if (== (Variables|Default|GetCurrentRandomCount) 3)
            _
            (else
              (switch int (LocalVariables|GetRandomIndex)
                (:Default
                  (goto _label_2))
                (:0
                  (goto _label))
                (:1
                  (goto _label))
                (:2
                  (goto _label_2))
                (:3
                  _))))
          (CallFunction|SummonMonster 3))))))

(fn Hit
  (params (Damage :type Integer) (IsHitable :type Boolean))
  (if (<= (Variables|Default|GetHitTimer) 0.0)
    (Variables|Default|SetHitTimer 0.5)))

(fn MeleeAttack
  (Variables|Default|SetIsMeleeAttack true)
  (Variables|Default|SetMaxSpeed 8e+02)
  (Rendering|Material|SetMaterial (Variables|Default|GetCube) 0 "/Game/Materials/M_Debug_Red.M_Debug_Red")
  (Utilities|Time|SetTimerbyFunctionName 0 "MeleeChaseEnd" 5.0))

(fn OnMeleeStart
  (Rendering|Material|SetMaterial (Variables|Default|GetCube) 0 "/Engine/BasicShapes/BasicShapeMaterial.BasicShapeMaterial")
  (CallFunction|StartRotate)
  (CallFunction|MeleeChaseEnd))

(fn MeleeChaseEnd
  (Rendering|Material|SetMaterial (Variables|Default|GetCube) 0 "/Engine/BasicShapes/BasicShapeMaterial.BasicShapeMaterial")
  (Variables|Default|SetIsMeleeAttack false)
  (Variables|Default|SetMaxSpeed 3e+02))

(fn RandomChooseStops
  (params (RandomCount :type Integer))
  (bind _output_get (LocalVariables|SetStops (Variables|Default|GetStops)))
  (for _index (range 1 RandomCount)
    (bind _output_get_2 (LocalVariables|SetThis (.OutItem (Utilities|Array|Random (Variables|Default|GetStops)))))
    (Utilities|Array|RemoveItem _output_get _output_get_2)
    (Default|Show _output_get_2)))

(fn HideAllStops
  (for _array_element (Variables|Default|GetStops)
    (Default|Hide _array_element)))

(fn MeleeCheck
  (if (Variables|Default|GetIsMeleeAttack)
    (Variables|Default|SetTarget%20Location (Transformation|GetActorLocation (Game|Player|GetPlayerPawn 0)))
    (if (Variables|Default|GetIsCloseEnough)
      (CallFunction|OnMeleeStart))))

(fn LazerChase
  (if (Variables|Default|GetIsShooingLazer)
    (bind _asbp_third_person_character_base (Utilities|Casting|CastToBP_ThirdPersonCharacter_Base (Game|Player|GetPlayerPawn 0)))
    (Variables|Default|SetLazerTarget (Math|Interpolation|VInterpTo (Variables|Default|GetLazerTarget) (Transformation|GetWorldLocation (Variables|/Game/Characters/BP_ThirdPersonCharacter_Base.BP_ThirdPersonCharacter_Base_C|GetSphere _asbp_third_person_character_base)) (Variables|Default|GetDelta%20Seconds) 5.0))
    (bind _ishit (CallFunction|ShootLazer (Transformation|GetWorldLocation (Variables|Default|GetEye1)) (Variables|Default|GetLazerTarget)))
    (bind _ishit_2 (CallFunction|ShootLazer (Transformation|GetWorldLocation (Variables|Default|GetEye2)) (Variables|Default|GetLazerTarget)))
    (if (or _ishit _ishit_2)
      (CallFunction|Hit 20 false))))

(fn BasicMovement
  (bind _pivot (Variables|Default|GetPivot))
  (bind _target_location (Variables|Default|GetTarget%20Location))
  (bind _returnvalue (Transformation|GetWorldLocation _pivot))
  (bind _returnvalue_2 (Math|Vector|Distance(Vector) _target_location _returnvalue))
  (bind _movedirection (CallFunction|GetFlyingMoveDirection (Variables|Default|GetTarget%20Location)))
  (Variables|Default|SetTarget%20Direction _movedirection)
  (Development|PrintString (Utilities|String|ToString(Float) _returnvalue_2) true true "(R=0.000000,G=0.660000,B=1.000000,A=1.000000)" (Variables|Default|GetDelta%20Seconds))
  (bind _output_get (Variables|Default|SetIsCloseEnough (<= _returnvalue_2 5e+01)))
  (if _output_get
    (CallFunction|RandomMovement)
    (else
      (bind _output_get_2 (Variables|Default|SetVelocity (Math|Interpolation|VInterpTo (Variables|Default|GetVelocity) (* (Variables|Default|GetTarget%20Direction) (Variables|Default|GetMaxSpeed)) (Variables|Default|GetDelta%20Seconds) 5.0)))
      (bind _sweephitresult (Transformation|AddActorWorldOffset (* (Variables|Default|GetDelta%20Seconds) _output_get_2)))
      (Utilities|IsValid (.HitActor (Collision|BreakHitResult _sweephitresult))
        (:Is%20Valid
          (CallFunction|RandomMovement))))))

(fn SummonMonster
  (params (Number :type Integer))
  (bind _returnvalue (Transformation|GetActorLocation))
  (bind _flyingarea (Variables|Default|GetFlyingArea))
  (bind _randomlocation (Default|GetRandomPoint _flyingarea))
  (bind _returnvalue_2 (Math|Vector|MakeVector (.x _randomlocation) (.y _randomlocation) (.z _returnvalue)))
  (for _index (range 1 Number)
    (bind _returnvalue_3 (Game|SpawnActorfromClass "/Game/Enemies/Eye_Test/BP_Eye_Monster.BP_Eye_Monster_C" (Math|Transform|MakeTransform _returnvalue_2 (Math|Rotator|FindLookatRotation _returnvalue_2 (Transformation|GetActorLocation (Game|Player|GetPlayerPawn 0)))) "Undefined" "MultiplyWithRoot" 0 0))
    (Utilities|Array|Add (Variables|Default|GetSummonedEnemy) _returnvalue_3)))

(fn EnemyCheck
  (for _array_element (Variables|Default|GetSummonedEnemy)
    (Utilities|IsValid _array_element
      (:Is%20Not%20Valid
        (Utilities|Array|RemoveItem (Variables|Default|GetSummonedEnemy) _array_element)))))

(fn Rotate
  (bind _output_get (Variables|Default|SetCurrentAngle (- (Variables|Default|GetCurrentAngle) (* (Variables|Default|GetDelta%20Seconds) (Variables|Default|GetRotateSpeed)))))
  (Transformation|SetRelativeRotation (Variables|Default|GetPivot) (Math|Rotator|MakeRotator 0.0 0.0 _output_get) false false)
  (if (<= (Variables|Default|GetCurrentAngle) -3.6e+02)
    (Variables|Default|SetIsRotating false)))

(fn Stun
  (CallFunction|Boss被Stun))

(fn Recover
  (CallFunction|BossRecover))

(fn GetIsStunned
  (return (Variables|玩家交互|GetIs%20Stunned)))