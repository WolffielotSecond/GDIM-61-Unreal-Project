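; Boss-fight actor, named as a laser stop, whose cube moves vertically between a shown and a hidden height.
; Show and Hide set the target height and switch the cube to query-only collision.
; Tick interpolates Z toward that target at ShowSpeed in both directions, without sweeping, and restores query-and-physics collision once nearly there, whether shown or hidden.
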(event Custom|Show
  (Variables|Default|SetTargetHeight (Variables|Default|GetShowHeight))
  (Collision|SetCollisionEnabled (Variables|Default|GetCube) "QueryOnly"))

(event Custom|Hide
  (Variables|Default|SetTargetHeight (Variables|Default|GetHideHeight))
  (Collision|SetCollisionEnabled (Variables|Default|GetCube) "QueryOnly"))

(event EventTick
  (params (DeltaSeconds :type Float%20%28single-precision%29))
  (bind _returnvalue (Transformation|GetActorLocation))
  (bind (_x _y _z) (Math|Vector|BreakVector _returnvalue))
  (Transformation|SetActorLocation (Math|Vector|MakeVector _x _y (Math|Interpolation|FInterpTo _z (Variables|Default|GetTargetHeight) DeltaSeconds (Variables|Default|GetShowSpeed))) false false)
  (if (Math|Float|NearlyEqual(Float) (.z (Transformation|GetActorLocation)) (Variables|Default|GetTargetHeight) 0.08)
    (Collision|SetCollisionEnabled (Variables|Default|GetCube) "QueryAndPhysics")))

(fn ConstructionScript)