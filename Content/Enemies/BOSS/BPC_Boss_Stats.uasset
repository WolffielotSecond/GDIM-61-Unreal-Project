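; Actor component holding the health and tenacity stats of the boss AI, caching its BP_AI_BOSS owner on BeginPlay.
; Damage lowers health and triggers the boss death event on the owner when health reaches zero or below.
; Tenacity hits accumulate only while the boss is not stunned, triggering the boss's stun when they reach the maximum.
; A separate event resets tenacity to zero.
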(event Custom|扣血
  (params (上海 :type Float%20%28double-precision%29))
  (Variables|Default|SetHealth (- (Variables|Default|GetHealth) 上海))
  (CallFunction|是否撕掉))

(event Custom|是否撕掉
  (if (<= (Variables|Default|GetHealth) 0.0)
    (CallFunction|撕掉)))

(event Custom|撕掉
  (Default|Boss死亡 (Variables|Default|GetBoss%20Ref)))

(event Custom|扣韧
  (params (韧性（正的数值） :type Float%20%28double-precision%29))
  (if (not (Variables|/Game/Enemies/BOSS/BP_AI_BOSS.BP_AI_BOSS_C|GetIs%20Stunned (Variables|Default|GetBoss%20Ref)))
    (Variables|Default|SetTenacity (+ 韧性（正的数值） (Variables|Default|GetTenacity)))
    (CallFunction|是否破防)))

(event Custom|是否破防
  (if (>= (Variables|Default|GetTenacity) (Variables|Default|GetMax%20Tenacity))
    (Default|Boss被Stun (Variables|Default|GetBoss%20Ref))))

(event Custom|恢复韧性值
  (Variables|Default|SetTenacity 0.0))

(event EventBeginPlay
  (bind _asbp_ai_boss (Utilities|Casting|CastToBP_AI_BOSS (Components|GetOwner)))
  (Variables|Default|SetBoss%20Ref _asbp_ai_boss))