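; Level load box for the Neuro02 to Vertical Slice 3 transition, with overrides for its overlap handling and condition check.
; On begin overlap it enables query and physics collision on the static meshes of its Actors list, and on end overlap it disables it.
; Its Condition passes when the Neuro02_SafeRoom streaming level is loaded and visible, otherwise it returns the custom game controller's LungActivated flag, and it debug-prints the level check.
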(event EventBeginPlay
  (|CallParentFunction) ; This node is disabled and will not be called.\nDrag off pins to build functionality.
)

(event Collision|EventActorBeginOverlap
  (params (OtherActor :type Actor%20Object%20Reference))
  (|CallParentFunction OtherActor) ; This node is disabled and will not be called.\nDrag off pins to build functionality.
)

(event EventTick
  (params (DeltaSeconds :type Float%20%28single-precision%29))
  (|CallParentFunction DeltaSeconds) ; This node is disabled and will not be called.\nDrag off pins to build functionality.
)

(event EventBeginOverlapOverride
  (for _array_element (Variables|Default|GetActors)
    (Collision|SetCollisionEnabled (Variables|/Script/Engine.StaticMeshActor|GetStaticMeshComponent _array_element) "QueryAndPhysics")))

(event EventEndOverlapOverride
  (for _array_element (Variables|Default|GetActors)
    (Collision|SetCollisionEnabled (Variables|/Script/Engine.StaticMeshActor|GetStaticMeshComponent _array_element) "NoCollision")))

(fn ConstructionScript
  (|CallParentFunction))

(fn Condition
  (bind _returnvalue (Class|GameplayStatics|GetStreamingLevel "Neuro02_SafeRoom"))
  (bind _returnvalue_2 (Class|LevelStreaming|IsLevelVisible _returnvalue))
  (bind _returnvalue_3 (Class|LevelStreaming|IsLevelLoaded _returnvalue))
  (bind _returnvalue_4 (and _returnvalue_2 _returnvalue_3))
  (Development|PrintString (Utilities|String|ToString(Boolean) _returnvalue_4))
  (if _returnvalue_4
    (return true)
    (else
      (bind _asbp_custom_game_controller (Utilities|Casting|CastToBP_Custom_GameController (Game|GetPlayerController 0)))
      (return (Variables|/Game/Blueprints/BP_Custom_GameController.BP_Custom_GameController_C|GetLung%20Activated _asbp_custom_game_controller)))))