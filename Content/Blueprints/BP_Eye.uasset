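; BP_Eye is a sentry eye that cycles between closed and open on a timer and goes on alert when it sees the player.
; An overlap box stores the player reference and enables a per-tick, debug-drawn visibility trace to the player's sphere while the eye is open.
; A hit refreshes the alert timer; expiry drops alert back to open, then closed.
; Cube debug materials show each state.
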(event OnComponentBeginOverlap(PlayerDetectionBox)
  (params (OverlappedComponent :type Primitive%20Component%20Object%20Reference) (OtherActor :type Actor%20Object%20Reference) (OtherComp :type Primitive%20Component%20Object%20Reference) (OtherBodyIndex :type Integer) (bFromSweep :type Boolean) (SweepResult :type Hit%20Result%20Structure%20%28by%20ref%29))
  (if (Actor|ActorHasTag OtherActor "Player")
    (bind _asbp_third_person_character_base (Utilities|Casting|CastToBP_ThirdPersonCharacter_Base OtherActor))
    (Variables|Default|SetPlayer%20Ref _asbp_third_person_character_base)
    (Variables|Default|SetShould%20Do%20Detection%20Trace true)))

(event OnComponentEndOverlap(PlayerDetectionBox)
  (params (OverlappedComponent :type Primitive%20Component%20Object%20Reference) (OtherActor :type Actor%20Object%20Reference) (OtherComp :type Primitive%20Component%20Object%20Reference) (OtherBodyIndex :type Integer))
  (if (Actor|ActorHasTag OtherActor "Player")
    (Variables|Default|SetShould%20Do%20Detection%20Trace false)
    (Variables|Default|SetPlayer%20Ref 0)))

(event EventTick
  (params (DeltaSeconds :type Float%20%28single-precision%29))
  (Utilities|FlowControl|Sequence
    (:then_0
      (if (and (Variables|Default|GetShould%20Do%20Detection%20Trace) (Variables|Default|GetEye%20Opened))
        (bind _player_ref (Variables|Default|GetPlayer%20Ref)
          (:then
            (bind _outhit (Collision|LineTraceByChannel (Transformation|GetWorldLocation (Variables|Default|GetEye%20Start%20Location)) (Transformation|GetWorldLocation (Variables|/Game/Characters/BP_ThirdPersonCharacter_Base.BP_ThirdPersonCharacter_Base_C|GetSphere _player_ref)) "TraceTypeQuery1" false 0 "ForOneFrame"))
            (if (Actor|ActorHasTag (.HitActor (Collision|BreakHitResult _outhit)) "Player")
              (Variables|Default|SetDetected%20Something true)))
          (:else))))
    (:then_1
      (Variables|Default|SetTimer (- (Variables|Default|GetTimer) (Utilities|Time|GetWorldDeltaSeconds))))
    (:then_2
      (if (Variables|Default|GetEye%20Opened)
        (if (Variables|Default|GetDetected%20Something)
          (Variables|Default|SetTimer 5.0)
          (Variables|Default|SetDetected%20Something false)
          (Variables|Default|SetOn%20Alert true)
          (Rendering|Material|SetMaterial (Variables|Default|GetCube) 0 (Variables|Debug|GetDebug%20Red))
          (elif (Variables|Default|GetOn%20Alert)
            (if (<= (Variables|Default|GetTimer) 0.0)
              (Variables|Default|SetTimer 5.0)
              (Variables|Default|SetOn%20Alert false)
              (Rendering|Material|SetMaterial (Variables|Default|GetCube) 0 (Variables|Debug|GetDebug%20Green)))
            (elif (<= (Variables|Default|GetTimer) 0.0)
              (Variables|Default|SetTimer 5.0)
              (Variables|Default|SetEye%20Opened false)
              (Rendering|Material|SetMaterial (Variables|Default|GetCube) 0 (Variables|Debug|GetDebug%20Gray)))))
        (elif (<= (Variables|Default|GetTimer) 0.0)
          (Variables|Default|SetTimer 5.0)
          (Variables|Default|SetEye%20Opened true)
          (Rendering|Material|SetMaterial (Variables|Default|GetCube) 0 (Variables|Debug|GetDebug%20Green)))))))

(fn ConstructionScript)