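; Level edge trigger box that controls whether the camera follows the player at the side boundaries of a level.
; On overlap, a dot product of the player's forward and a right vector, checked against IsLeftLevel, decides whether to stop camera follow.
; Leaving the box restores following and sets HasEnteredBefore, which also starts true for the initial level.
; Level streaming logic gated by terminal or easter-egg state is disconnected and never runs.
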(event OnComponentBeginOverlap(Box)
  (params (OverlappedComponent :type Primitive%20Component%20Object%20Reference) (OtherActor :type Actor%20Object%20Reference) (OtherComp :type Primitive%20Component%20Object%20Reference) (OtherBodyIndex :type Integer) (bFromSweep :type Boolean) (SweepResult :type Hit%20Result%20Structure%20%28by%20ref%29))
  (if (Actor|ActorHasTag OtherActor "Player")
    (if (Variables|Default|GetIs%20Left%20Level)
      (if (> (Math|Vector|DotProduct (Class|KismetMathLibrary|VectorRight) (Transformation|GetActorForwardVector (Game|GetPlayerCharacter 0))) 0.0)
        (Variables|/Game/Blueprints/BP_Camera.BP_Camera_C|SetCamera%20Should%20Follow%20Player (Variables|/Game/Characters/BP_ThirdPersonCharacter_Base.BP_ThirdPersonCharacter_Base_C|GetCamera%20Actor%20Reference (Variables|Default|GetPlayer%20Ref)) false))
      (elif (not (> (Math|Vector|DotProduct (Class|KismetMathLibrary|VectorRight) (Transformation|GetActorForwardVector (Game|GetPlayerCharacter 0))) 0.0))
        (Variables|/Game/Blueprints/BP_Camera.BP_Camera_C|SetCamera%20Should%20Follow%20Player (Variables|/Game/Characters/BP_ThirdPersonCharacter_Base.BP_ThirdPersonCharacter_Base_C|GetCamera%20Actor%20Reference (Variables|Default|GetPlayer%20Ref)) false)))))

(event OnComponentEndOverlap(Box)
  (params (OverlappedComponent :type Primitive%20Component%20Object%20Reference) (OtherActor :type Actor%20Object%20Reference) (OtherComp :type Primitive%20Component%20Object%20Reference) (OtherBodyIndex :type Integer))
  (if (Actor|ActorHasTag OtherActor "Player")
    (Variables|/Game/Blueprints/BP_Camera.BP_Camera_C|SetCamera%20Should%20Follow%20Player (Variables|/Game/Characters/BP_ThirdPersonCharacter_Base.BP_ThirdPersonCharacter_Base_C|GetCamera%20Actor%20Reference (Variables|Default|GetPlayer%20Ref)) true)
    (Variables|Default|SetHas%20Entered%20Before true)))

(event EventBeginPlay
  (bind _asbp_custom_gamemode (Utilities|Casting|CastToBP_Custom_Gamemode (Game|GetGameMode)))
  (Variables|Default|SetGamemode%20Ref _asbp_custom_gamemode)
  (bind _asbp_third_person_character_base (Utilities|Casting|CastToBP_ThirdPersonCharacter_Base (Game|GetPlayerCharacter 0)))
  (Variables|Default|SetPlayer%20Ref _asbp_third_person_character_base)
  (if (Variables|Default|GetIs%20Initial%20Level)
    (Variables|Default|SetHas%20Entered%20Before true)))

(fn ConstructionScript)