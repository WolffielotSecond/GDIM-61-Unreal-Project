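; BP_Wind_Distortions is a static world object with two planes, named for wind distortion, that appear only when the player's Lung is activated.
; On BeginPlay it reads LungActivated from BP_Custom_GameController and shows or hides both planes to match.
; An OnLungActivated event reveals both planes later, with no matching event to hide them again.
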(event EventBeginPlay
  (bind _asbp_custom_game_controller (Utilities|Casting|CastToBP_Custom_GameController (Game|GetPlayerController 0)))
  (if (Variables|/Game/Blueprints/BP_Custom_GameController.BP_Custom_GameController_C|GetLung%20Activated _asbp_custom_game_controller)
    (Rendering|SetVisibility (Variables|Default|GetPlane1) true false)
    (Rendering|SetVisibility (Variables|Default|GetPlane) true false)
    (else
      (Rendering|SetVisibility (Variables|Default|GetPlane) false false)
      (Rendering|SetVisibility (Variables|Default|GetPlane1) false false))))

(event EventOnLungActivated
  (Rendering|SetVisibility (Variables|Default|GetPlane1) true false)
  (Rendering|SetVisibility (Variables|Default|GetPlane) true false))

(fn ConstructionScript)