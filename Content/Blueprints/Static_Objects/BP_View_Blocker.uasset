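; View blocker static object whose cube material changes opacity while the player is inside its box trigger.
; BeginPlay builds a dynamic material instance from configurable base color, metallic, roughness and normal textures, then applies it to the cube.
; Box overlaps with a Player-tagged character's capsule toggle a flag.
; Tick ramps the Opacity parameter toward TimerHead while the flag is set and back to zero otherwise.
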(event OnComponentBeginOverlap(Box)
  (params (OverlappedComponent :type Primitive%20Component%20Object%20Reference) (OtherActor :type Actor%20Object%20Reference) (OtherComp :type Primitive%20Component%20Object%20Reference) (OtherBodyIndex :type Integer) (bFromSweep :type Boolean) (SweepResult :type Hit%20Result%20Structure%20%28by%20ref%29))
  (bind _ascharacter (Utilities|Casting|CastToCharacter OtherActor))
  (if (and (== OtherComp (Variables|/Script/Engine.Character|GetCapsuleComponent _ascharacter)) (Actor|ActorHasTag OtherActor "Player"))
    (Variables|Default|SetPlayer%20Exposed true)))

(event OnComponentEndOverlap(Box)
  (params (OverlappedComponent :type Primitive%20Component%20Object%20Reference) (OtherActor :type Actor%20Object%20Reference) (OtherComp :type Primitive%20Component%20Object%20Reference) (OtherBodyIndex :type Integer))
  (bind _ascharacter (Utilities|Casting|CastToCharacter OtherActor))
  (if (and (== OtherComp (Variables|/Script/Engine.Character|GetCapsuleComponent _ascharacter)) (Actor|ActorHasTag OtherActor "Player"))
    (Variables|Default|SetPlayer%20Exposed false)))

(event EventBeginPlay
  (bind _returnvalue (Rendering|Material|CreateDynamicMaterialInstance "/Game/Materials/View_Blocking_Materials/M_VIewBlocker_Parent.M_VIewBlocker_Parent" "None" "None" :!class /Script/Engine.KismetMaterialLibrary))
  (Variables|Default|SetMaterial _returnvalue)
  (bind _basic_color (Variables|Default|GetBasic%20Color)
    (:then
      (Rendering|Material|SetTextureParameterValue (Variables|Default|GetMaterial) "Basic_Color" _basic_color))
    (:else
      _))
  (bind _metallic (Variables|Default|GetMetallic)
    (:then
      (Rendering|Material|SetTextureParameterValue (Variables|Default|GetMaterial) "Metallic" _metallic))
    (:else
      _))
  (bind _roughness (Variables|Default|GetRoughness)
    (:then
      (Rendering|Material|SetTextureParameterValue (Variables|Default|GetMaterial) "Roughness" _roughness))
    (:else
      _))
  (bind _normal (Variables|Default|GetNormal)
    (:then
      (Rendering|Material|SetTextureParameterValue (Variables|Default|GetMaterial) "Normal" _normal)
      (Rendering|Material|SetScalarParameterValue (Variables|Default|GetMaterial) "Opacity" 0.0 :!class /Script/Engine.MaterialInstanceDynamic))
    (:else
      _))
  (Rendering|Material|SetMaterial (Variables|Default|GetCube) (Variables|Default|GetMaterial%20Index) (Variables|Default|GetMaterial)))

(event EventTick
  (params (DeltaSeconds :type Float%20%28single-precision%29))
  (if (Variables|Default|GetPlayer%20Exposed)
    (if (>= (Variables|Default|GetTimer) (Variables|Default|GetTimer%20Head))
      (bind _output_get (Variables|Default|SetTimer (Variables|Default|GetTimer%20Head)))
      (Rendering|Material|SetScalarParameterValue (Variables|Default|GetMaterial) "Opacity" _output_get :!class /Script/Engine.MaterialInstanceDynamic)
      (else
        (bind _output_get_2 (Variables|Default|SetTimer (+ (Variables|Default|GetTimer) (* (Utilities|Time|GetWorldDeltaSeconds) 2.0))))
        (Rendering|Material|SetScalarParameterValue (Variables|Default|GetMaterial) "Opacity" _output_get_2 :!class /Script/Engine.MaterialInstanceDynamic)))
    (elif (<= (Variables|Default|GetTimer) 0.0)
      (bind _output_get_3 (Variables|Default|SetTimer 0.0))
      (Rendering|Material|SetScalarParameterValue (Variables|Default|GetMaterial) "Opacity" _output_get_3 :!class /Script/Engine.MaterialInstanceDynamic)
      (else
        (bind _output_get_4 (Variables|Default|SetTimer (- (Variables|Default|GetTimer) (* (Utilities|Time|GetWorldDeltaSeconds) 2.0))))
        (Rendering|Material|SetScalarParameterValue (Variables|Default|GetMaterial) "Opacity" _output_get_4 :!class /Script/Engine.MaterialInstanceDynamic)))))

(fn ConstructionScript)