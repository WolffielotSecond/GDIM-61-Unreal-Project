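; BP_DrawBridge_Self is a drawbridge that drops by physics when its Fall event is called.
; At BeginPlay, the pre-fall constraint colliders are solid, while the landing ground and fallen-position walls have collision off.
; Fall turns on the landing colliders and simulates physics on the Cube for two seconds, then freezes it and disables the pre-fall colliders.
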(event Custom|Fall
  (Collision|SetCollisionEnabled (Variables|Default|GetConstraint%20Wall%202) "QueryAndPhysics")
  (Collision|SetCollisionEnabled (Variables|Default|GetConstraint%20Wall) "QueryAndPhysics")
  (Collision|SetCollisionEnabled (Variables|Default|GetLand%20Ground) "QueryAndPhysics")
  (Physics|SetSimulatePhysics (Variables|Default|GetCube) true)
  (Utilities|FlowControl|Delay 2.0)
  (Physics|SetSimulatePhysics (Variables|Default|GetCube) false)
  (Collision|SetCollisionEnabled (Variables|Default|GetConstraint_Prefall) "NoCollision")
  (Collision|SetCollisionEnabled (Variables|Default|GetConstraint%20Wall_Prefall) "NoCollision")
  (Collision|SetCollisionEnabled (Variables|Default|GetConstraint%20Wall_Prefall2) "NoCollision"))

(event EventBeginPlay
  (Collision|SetCollisionEnabled (Variables|Default|GetLand%20Ground) "NoCollision")
  (Collision|SetCollisionEnabled (Variables|Default|GetConstraint%20Wall%202) "NoCollision")
  (Collision|SetCollisionEnabled (Variables|Default|GetConstraint%20Wall) "NoCollision")
  (Collision|SetCollisionEnabled (Variables|Default|GetConstraint_Prefall) "QueryAndPhysics")
  (Collision|SetCollisionEnabled (Variables|Default|GetConstraint%20Wall_Prefall) "QueryAndPhysics")
  (Collision|SetCollisionEnabled (Variables|Default|GetConstraint%20Wall_Prefall2) "QueryAndPhysics"))

(fn ConstructionScript)