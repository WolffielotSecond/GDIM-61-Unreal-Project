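; BP_Pusher is a map item that pushes player characters inside its Box trigger once the game controller's LungActivated state is on.
; On begin and end overlap it passes its Speed to the character's OnPusherTouch and OnPusherLeave, leaving the push itself to the character.
; Smoke turns on at BeginPlay if the lung is already active, or when OnLungActivated is called.
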(event OnComponentBeginOverlap(Box)
  (params (OverlappedComponent :type Primitive%20Component%20Object%20Reference) (OtherActor :type Actor%20Object%20Reference) (OtherComp :type Primitive%20Component%20Object%20Reference) (OtherBodyIndex :type Integer) (bFromSweep :type Boolean) (SweepResult :type Hit%20Result%20Structure%20%28by%20ref%29))
  (bind _game_comtroller (Variables|Default|GetGame%20Comtroller)
    (:then
      (if (Variables|/Game/Blueprints/BP_Custom_GameController.BP_Custom_GameController_C|GetLung%20Activated _game_comtroller)
        (bind _asbp_third_person_character_base (Utilities|Casting|CastToBP_ThirdPersonCharacter_Base OtherActor))
        (Default|OnPusherTouch _asbp_third_person_character_base (Variables|Default|GetSpeed))))
    (:else
      (Development|PrintString "No"))))

(event OnComponentEndOverlap(Box)
  (params (OverlappedComponent :type Primitive%20Component%20Object%20Reference) (OtherActor :type Actor%20Object%20Reference) (OtherComp :type Primitive%20Component%20Object%20Reference) (OtherBodyIndex :type Integer))
  (bind _game_comtroller (Variables|Default|GetGame%20Comtroller)
    (:then
      (if (Variables|/Game/Blueprints/BP_Custom_GameController.BP_Custom_GameController_C|GetLung%20Activated _game_comtroller)
        (bind _asbp_third_person_character_base (Utilities|Casting|CastToBP_ThirdPersonCharacter_Base OtherActor))
        (Default|OnPusherLeave _asbp_third_person_character_base (Variables|Default|GetSpeed))))
    (:else
      (Development|PrintString "No"))))

(event EventBeginPlay
  (bind _asbp_custom_game_controller (Utilities|Casting|CastToBP_Custom_GameController (Game|GetPlayerController 0))
    (:then
      (bind _output_get (Variables|Default|SetGame%20Comtroller _asbp_custom_game_controller))
      (if (Variables|/Game/Blueprints/BP_Custom_GameController.BP_Custom_GameController_C|GetLung%20Activated _output_get)
        (Components|Activation|Activate (Variables|Default|GetSmoke) false)))
    (:CastFailed
      (Development|PrintString "failed"))))

(event EventOnLungActivated
  (Components|Activation|Activate (Variables|Default|GetSmoke) false))

(fn ConstructionScript)