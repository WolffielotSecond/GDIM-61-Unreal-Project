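; BP_Accelerator is a map item that pushes the player along its forward direction at a set speed.
; Box overlaps with the character's capsule switch the push on and off, only while the game controller's LungActivated flag is set.
; Tick offsets the player without sweeping, and continues after a jumping exit until OnLand clears the jump flag.
; On entry, it passes itself to the character through OnAcceleratorTouch.
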(event OnComponentEndOverlap(Box)
  (params (OverlappedComponent :type Primitive%20Component%20Object%20Reference) (OtherActor :type Actor%20Object%20Reference) (OtherComp :type Primitive%20Component%20Object%20Reference) (OtherBodyIndex :type Integer))
  (bind _game_comtroller (Variables|Default|GetGame%20Comtroller)
    (:then
      (if (Variables|/Game/Blueprints/BP_Custom_GameController.BP_Custom_GameController_C|GetLung%20Activated _game_comtroller)
        (bind _asbp_third_person_character_base (Utilities|Casting|CastToBP_ThirdPersonCharacter_Base OtherActor))
        (if (== OtherComp (Variables|/Script/Engine.Character|GetCapsuleComponent _asbp_third_person_character_base))
          (Variables|Default|SetIsOn false)
          (if (Variables|/Script/Engine.Character|GetbWasJumping _asbp_third_person_character_base)
            (Variables|Default|SetIsJump true)))))
    (:else)))

(event OnComponentBeginOverlap(Box)
  (params (OverlappedComponent :type Primitive%20Component%20Object%20Reference) (OtherActor :type Actor%20Object%20Reference) (OtherComp :type Primitive%20Component%20Object%20Reference) (OtherBodyIndex :type Integer) (bFromSweep :type Boolean) (SweepResult :type Hit%20Result%20Structure%20%28by%20ref%29))
  (bind _game_comtroller (Variables|Default|GetGame%20Comtroller)
    (:then
      (if (Variables|/Game/Blueprints/BP_Custom_GameController.BP_Custom_GameController_C|GetLung%20Activated _game_comtroller)
        (bind _asbp_third_person_character_base (Utilities|Casting|CastToBP_ThirdPersonCharacter_Base OtherActor))
        (Variables|Default|SetPlayer _asbp_third_person_character_base)
        (if (== OtherComp (Variables|/Script/Engine.Character|GetCapsuleComponent _asbp_third_person_character_base))
          (Default|OnAcceleratorTouch _asbp_third_person_character_base self)
          (Variables|Default|SetIsOn true))))
    (:else
      (Development|PrintString "No"))))

(event EventBeginPlay
  (bind _asbp_custom_game_controller (Utilities|Casting|CastToBP_Custom_GameController (Game|GetPlayerController 0)))
  (Variables|Default|SetGame%20Comtroller _asbp_custom_game_controller))

(event EventTick
  (params (DeltaSeconds :type Float%20%28single-precision%29))
  (if (or (Variables|Default|GetIsOn) (Variables|Default|GetIsJump))
    (Transformation|AddActorWorldOffset (Variables|Default|GetPlayer) (* (Math|Vector|GetForwardVector (Variables|Default|GetDefaultSceneRoot)) (Variables|Default|GetSpeed) DeltaSeconds))))

(event EventOnLand
  (Variables|Default|SetIsJump false))

(fn ConstructionScript)

(fn OnAcceleratorTouch
  (params (TargetAccelerator :type BP%20Accelerator%20Object%20Reference)))