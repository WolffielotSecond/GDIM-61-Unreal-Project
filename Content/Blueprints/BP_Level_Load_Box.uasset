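; Trigger box actor that streams levels in and out as the player passes through it.
; On overlap by an actor tagged "Player", it loads two soft-referenced levels without blocking, then unloads one, plus a second if that reference is valid.
; It fires on every overlap, as the DoOnce gate is disconnected, along with older array-based load loops.
; BeginPlay caches a player character reference that the overlap logic does not use.
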(event OnComponentBeginOverlap(Box)
  (params (OverlappedComponent :type Primitive%20Component%20Object%20Reference) (OtherActor :type Actor%20Object%20Reference) (OtherComp :type Primitive%20Component%20Object%20Reference) (OtherBodyIndex :type Integer) (bFromSweep :type Boolean) (SweepResult :type Hit%20Result%20Structure%20%28by%20ref%29))
  (if (Actor|ActorHasTag OtherActor "Player")
    (Class|GameplayStatics|LoadStreamLevelbySoftObjectPtr (Variables|Default|GetLoad%20Level%201%20Ref) true false)
    (Class|GameplayStatics|LoadStreamLevelbySoftObjectPtr (Variables|Default|GetLoad%20Level%202%20Ref) true false)
    (Class|GameplayStatics|UnloadStreamLevelbySoftObjectPtr (Variables|Default|GetUnload%20Level%201%20Ref) false)
    (bind _unload_level_2_ref (Variables|Default|GetUnload%20Level%202%20Ref)
      (:then
        (Class|GameplayStatics|UnloadStreamLevelbySoftObjectPtr _unload_level_2_ref false))
      (:else))))

(event EventBeginPlay
  (bind _asbp_third_person_character_base (Utilities|Casting|CastToBP_ThirdPersonCharacter_Base (Game|GetPlayerCharacter 0)))
  (Variables|Default|SetPlayer%20Ref _asbp_third_person_character_base))

(event Collision|EventActorBeginOverlap
  (params (OtherActor :type Actor%20Object%20Reference)))

(event EventTick
  (params (DeltaSeconds :type Float%20%28single-precision%29)))

(fn ConstructionScript)