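; Trigger volume that disables jumping for the third-person character while it is inside the Box.
; Capsule begin and end overlaps clear and restore the character's JumpIsNotLockedByScript flag and update CharacterInBox.
; Shortly after BeginPlay, an overlap check also locks jump if the player already starts inside, without setting CharacterInBox.
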(event OnComponentBeginOverlap(Box)
  (params (OverlappedComponent :type Primitive%20Component%20Object%20Reference) (OtherActor :type Actor%20Object%20Reference) (OtherComp :type Primitive%20Component%20Object%20Reference) (OtherBodyIndex :type Integer) (bFromSweep :type Boolean) (SweepResult :type Hit%20Result%20Structure%20%28by%20ref%29))
  (bind _asbp_third_person_character_base (Utilities|Casting|CastToBP_ThirdPersonCharacter_Base OtherActor))
  (if (== (Variables|/Script/Engine.Character|GetCapsuleComponent _asbp_third_person_character_base) OtherComp)
    (Variables|Default|SetCharacter%20In%20Box true)
    (Variables|/Game/Characters/BP_ThirdPersonCharacter_Base.BP_ThirdPersonCharacter_Base_C|SetJump%20Is%20Not%20Locked%20By%20Script _asbp_third_person_character_base false)))

(event OnComponentEndOverlap(Box)
  (params (OverlappedComponent :type Primitive%20Component%20Object%20Reference) (OtherActor :type Actor%20Object%20Reference) (OtherComp :type Primitive%20Component%20Object%20Reference) (OtherBodyIndex :type Integer))
  (bind _asbp_third_person_character_base (Utilities|Casting|CastToBP_ThirdPersonCharacter_Base OtherActor))
  (if (== (Variables|/Script/Engine.Character|GetCapsuleComponent _asbp_third_person_character_base) OtherComp)
    (Variables|Default|SetCharacter%20In%20Box false)
    (Variables|/Game/Characters/BP_ThirdPersonCharacter_Base.BP_ThirdPersonCharacter_Base_C|SetJump%20Is%20Not%20Locked%20By%20Script _asbp_third_person_character_base true)))

(event EventBeginPlay
  (Utilities|FlowControl|Delay 0.05)
  (if (Collision|IsOverlappingActor (Variables|Default|GetBox) (Game|GetPlayerCharacter 0) :!class /Script/Engine.PrimitiveComponent)
    (bind _asbp_third_person_character_base (Utilities|Casting|CastToBP_ThirdPersonCharacter_Base (Game|GetPlayerCharacter 0)))
    (Variables|/Game/Characters/BP_ThirdPersonCharacter_Base.BP_ThirdPersonCharacter_Base_C|SetJump%20Is%20Not%20Locked%20By%20Script _asbp_third_person_character_base false)))

(fn ConstructionScript)