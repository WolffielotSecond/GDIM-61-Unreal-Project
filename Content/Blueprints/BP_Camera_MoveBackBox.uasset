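; BP_Camera_MoveBackBox is a trigger volume that adjusts the third-person camera while a player character is inside it.
; When the character's capsule enters DetectionBox, it sends the box's arm length and Y offset to the character's camera actor and resizes that camera's auto-targeting sphere (自动索敌圈).
; When the capsule leaves, it restores hardcoded default values rather than the camera's previous settings.
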(event OnComponentBeginOverlap(DetectionBox)
  (params (OverlappedComponent :type Primitive%20Component%20Object%20Reference) (OtherActor :type Actor%20Object%20Reference) (OtherComp :type Primitive%20Component%20Object%20Reference) (OtherBodyIndex :type Integer) (bFromSweep :type Boolean) (SweepResult :type Hit%20Result%20Structure%20%28by%20ref%29))
  (bind _asbp_third_person_character_base (Utilities|Casting|CastToBP_ThirdPersonCharacter_Base OtherActor))
  (if (== (Variables|/Script/Engine.Character|GetCapsuleComponent _asbp_third_person_character_base) OtherComp)
    (Default|SetTargetFOVChangeValues (Variables|/Game/Characters/BP_ThirdPersonCharacter_Base.BP_ThirdPersonCharacter_Base_C|GetCamera%20Actor%20Reference _asbp_third_person_character_base) (Variables|Default|GetTarget%20Arm%20Length) (Variables|Default|GetTarget%20Arm%20Y%20Location))
    (Components|Sphere|SetSphereRadius (Variables|/Game/Blueprints/BP_Camera.BP_Camera_C|Get自动索敌圈 (Variables|/Game/Characters/BP_ThirdPersonCharacter_Base.BP_ThirdPersonCharacter_Base_C|GetCamera%20Actor%20Reference _asbp_third_person_character_base)) (Variables|Default|GetSphere%20Radius) true)))

(event OnComponentEndOverlap(DetectionBox)
  (params (OverlappedComponent :type Primitive%20Component%20Object%20Reference) (OtherActor :type Actor%20Object%20Reference) (OtherComp :type Primitive%20Component%20Object%20Reference) (OtherBodyIndex :type Integer))
  (bind _asbp_third_person_character_base (Utilities|Casting|CastToBP_ThirdPersonCharacter_Base OtherActor))
  (if (== (Variables|/Script/Engine.Character|GetCapsuleComponent _asbp_third_person_character_base) OtherComp)
    (Default|SetTargetFOVChangeValues (Variables|/Game/Characters/BP_ThirdPersonCharacter_Base.BP_ThirdPersonCharacter_Base_C|GetCamera%20Actor%20Reference _asbp_third_person_character_base) 5e+02 182.0)
    (Components|Sphere|SetSphereRadius (Variables|/Game/Blueprints/BP_Camera.BP_Camera_C|Get自动索敌圈 (Variables|/Game/Characters/BP_ThirdPersonCharacter_Base.BP_ThirdPersonCharacter_Base_C|GetCamera%20Actor%20Reference _asbp_third_person_character_base)) 32.0 true)))

(event EventBeginPlay)

(event Collision|EventActorBeginOverlap
  (params (OtherActor :type Actor%20Object%20Reference)))

(event EventTick
  (params (DeltaSeconds :type Float%20%28single-precision%29)))

(fn ConstructionScript)