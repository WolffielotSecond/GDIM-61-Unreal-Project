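; Base trigger volume that shows a tutorial message to the player once, then removes itself.
; When an actor tagged Player overlaps the trigger, it checks PlayConditionMet, which returns false here and serves as the hook for child triggers.
; On a pass, a DoOnce fires PlayMessage, which sends the Tutorial and delay settings to the player character and destroys the actor.
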(event OnComponentBeginOverlap(TutorialTrigger)
  (params (OverlappedComponent :type Primitive%20Component%20Object%20Reference) (OtherActor :type Actor%20Object%20Reference) (OtherComp :type Primitive%20Component%20Object%20Reference) (OtherBodyIndex :type Integer) (bFromSweep :type Boolean) (SweepResult :type Hit%20Result%20Structure%20%28by%20ref%29))
  (if (Actor|ActorHasTag OtherActor "Player")
    (bind _can_play_tutorial (CallFunction|PlayConditionMet OtherActor OtherComp))
    (if _can_play_tutorial
      (Utilities|FlowControl|DoOnce false
        (:Completed
          (CallFunction|PlayMessage))))))

(event Custom|Play%20%20Message
  (Class|BPIPlayerInterface|PlayTutorialMessage(Message) (Game|GetPlayerCharacter 0) (Variables|Default|GetTutorial) (Variables|Default|GetHas%20Delay?) (Variables|Default|GetDelay%20Seconds))
  (Actor|DestroyActor))

(event EventBeginPlay)

(event Collision|EventActorBeginOverlap
  (params (OtherActor :type Actor%20Object%20Reference)))

(event EventTick
  (params (DeltaSeconds :type Float%20%28single-precision%29)))

(fn ConstructionScript)

(fn PlayConditionMet
  (params (Other%20Actor :type Actor%20Object%20Reference) (Other%20Component :type Primitive%20Component%20Object%20Reference))
  (return false))