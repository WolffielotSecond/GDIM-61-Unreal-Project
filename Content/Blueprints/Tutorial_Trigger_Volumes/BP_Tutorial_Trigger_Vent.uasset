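; BP_Tutorial_Trigger_Vent is a tutorial trigger volume, named for a vent tutorial, that supplies its own condition for playing.
; It overrides the play condition check to return the LungActivated flag from player 0's BP_Custom_GameController, ignoring the overlapping actor and component.
; The event graph holds only disabled stubs, so any other trigger behavior comes from the parent class.
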(event EventBeginPlay
  (|CallParentFunction) ; This node is disabled and will not be called.\nDrag off pins to build functionality.
)

(event Collision|EventActorBeginOverlap
  (params (OtherActor :type Actor%20Object%20Reference))
  (|CallParentFunction OtherActor) ; This node is disabled and will not be called.\nDrag off pins to build functionality.
)

(event EventTick
  (params (DeltaSeconds :type Float%20%28single-precision%29))
  (|CallParentFunction DeltaSeconds) ; This node is disabled and will not be called.\nDrag off pins to build functionality.
)

(fn ConstructionScript
  (|CallParentFunction))

(fn PlayConditionMet
  (params (Other%20Actor :type Actor%20Object%20Reference) (Other%20Component :type Primitive%20Component%20Object%20Reference))
  (bind _asbp_custom_game_controller (Utilities|Casting|CastToBP_Custom_GameController (Game|GetPlayerController 0)))
  (return (Variables|/Game/Blueprints/BP_Custom_GameController.BP_Custom_GameController_C|GetLung%20Activated _asbp_custom_game_controller)))