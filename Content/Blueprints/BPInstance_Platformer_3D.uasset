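; Game instance for a 3D platformer that tracks a syringe count as a Steam user stat.
; Init asynchronously requests the current Steam stats, though the count is never read back from them here.
; CheckSyringeCount adds to the count, writes and stores the stat, then prints the total if storing succeeds.
; ResetSyringeCount zeroes the count and saves it through the same event.
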(event EventInit
  (|RequestCurrentStatsAsync 1e+01))

(event EventCheckSyringeCount
  (params (Add%20Number :type Integer))
  (bind _returnvalue (Class|SteamProUserStats|GetSteamUserStats))
  (bind _output_get (Variables|Default|SetSyringe%20Count (+ Add%20Number (Variables|Default|GetSyringe%20Count))))
  (Class|SteamProUserStats|SetStatInt _returnvalue "_Syringe_Stats" _output_get)
  (bind _returnvalue_2 (Class|SteamProUserStats|StoreStats _returnvalue))
  (if _returnvalue_2
    (Development|PrintString (Utilities|String|ToString(Text) (Utilities|Text|FormatText "Achievement {number}" (Variables|Default|GetSyringe%20Count))))))

(event EventResetSyringeCount
  (Variables|Default|SetSyringe%20Count 0)
  (CallFunction|CheckSyringeCount))