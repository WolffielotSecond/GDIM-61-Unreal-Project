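; Demo-only trigger volume that shows the end-of-demo screen when the player reaches it.
; On BeginPlay it destroys itself unless the custom game controller is flagged as the end-of-year demo build.
; A Player-tagged overlap disables the volume's collision, briefly locks input, and creates the WB_Demo widget.
; Timed delays sequence its closing messages, then it plays the exit animation and pauses the game.
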(event OnComponentBeginOverlap(TriggerVolumn)
  (params (OverlappedComponent :type Primitive%20Component%20Object%20Reference) (OtherActor :type Actor%20Object%20Reference) (OtherComp :type Primitive%20Component%20Object%20Reference) (OtherBodyIndex :type Integer) (bFromSweep :type Boolean) (SweepResult :type Hit%20Result%20Structure%20%28by%20ref%29))
  (if (Actor|ActorHasTag OtherActor "Player")
    (Collision|SetCollisionEnabled (Variables|Default|GetTrigger%20Volumn) "NoCollision")
    (Input|DisableInput (Game|GetPlayerCharacter 0) (Game|GetPlayerController 0))
    (bind _returnvalue (UserInterface|CreateWidget "/Game/UI/Demo_UI/WB_Demo.WB_Demo_C" (Game|GetPlayerController 0)))
    (bind _output_get (Variables|Default|SetDemo _returnvalue))
    (UserInterface|Viewport|AddtoViewport _output_get 0)
    (Default|ShowAnimation _output_get)
    (Utilities|FlowControl|Delay 0.5)
    (Input|EnableInput (Game|GetPlayerCharacter 0) (Game|GetPlayerController 0))
    (Default|PlayOneSequenceOfAnimation (Variables|Default|GetDemo) "You’ve reached the end of the demo.")
    (Utilities|FlowControl|Delay 3.5)
    (Default|PlayOneSequenceOfAnimation (Variables|Default|GetDemo) "Thank you for playing.")
    (Utilities|FlowControl|Delay 3.5)
    (Default|ExitGameAnim (Variables|Default|GetDemo))
    (Game|SetGamePaused true)))

(event EventBeginPlay
  (bind _asbp_custom_game_controller (Utilities|Casting|CastToBP_Custom_GameController (Game|GetPlayerController 0)))
  (if (not (Variables|/Game/Blueprints/BP_Custom_GameController.BP_Custom_GameController_C|GetIs%20End%20Of%20Year%20Demo _asbp_custom_game_controller))
    (Actor|DestroyActor)))

(event Collision|EventActorBeginOverlap
  (params (OtherActor :type Actor%20Object%20Reference)))

(event EventTick
  (params (DeltaSeconds :type Float%20%28single-precision%29)))

(fn ConstructionScript)