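; BP_Demo_End_Actualizer runs the end-of-demo sequence as soon as it begins play.
; It briefly disables player input while creating the WB_Demo widget and showing its intro animation, then restores input.
; Timed delays step the widget through two closing messages before triggering its exit-game animation and pausing the game.
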(event EventBeginPlay
  (Input|DisableInput (Game|GetPlayerCharacter 0) (Game|GetPlayerController 0))
  (bind _returnvalue (UserInterface|CreateWidget "/Game/UI/Demo_UI/WB_Demo.WB_Demo_C" (Game|GetPlayerController 0)))
  (bind _output_get (Variables|Default|SetDemo _returnvalue))
  (UserInterface|Viewport|AddtoViewport _output_get 0)
  (Default|ShowAnimation _output_get)
  (Utilities|FlowControl|Delay 0.5)
  (Input|EnableInput (Game|GetPlayerCharacter 0) (Game|GetPlayerController 0))
  (Default|PlayOneSequenceOfAnimation (Variables|Default|GetDemo) "You’ve reached the end of the demo.")
  (Utilities|FlowControl|Delay 3.5)
  (Default|PlayOneSequenceOfAnimation (Variables|Default|GetDemo) "Thank you for playing.")
  (Utilities|FlowControl|Delay 3.5)
  (Default|ExitGameAnim (Variables|Default|GetDemo))
  (Game|SetGamePaused true))

(fn ConstructionScript)