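; Interactable door Blueprint for a vertical slice that can be blocked by vines.
; It overrides Interact and acts only once the door is Solved.
; While its DoorJammerReference is valid, it shows a vines-covered prompt through the player character; otherwise it calls SolvedInteraction.
; BeginPlay, overlap and Tick are disabled stubs, and construction defers to the parent.
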(event EventBeginPlay
  (|CallParentFunction) ; This node is disabled and will not be called.\nDrag off pins to build functionality.
)

(event Collision|EventActorBeginOverlap
  (params (OtherActor :type Actor%20Object%20Reference))
  (|CallParentFunction OtherActor) ; This node is disabled and will not be called.\nDrag off pins to build functionality.
)

(event EventTick
  (params (DeltaSeconds :type Float%20%28single-precision%29))
  (|CallParentFunction DeltaSeconds) ; This node is disabled and will not be called.\nDrag off pins to build functionality.
)

(event EventInteract
  (if (Variables|Default|GetSolved?)
    (Variables|Default|GetDoor%20Jammer%20Reference
      (:then
        (Class|BPIPlayerInterface|LookatPromptPlay(Message) (Game|GetPlayerCharacter 0) "The Door Is Covered With Vines"))
      (:else
        (CallFunction|SolvedInteraction)))))

(fn ConstructionScript
  (|CallParentFunction))