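; Easter-egg terminal interactable that reveals a keyboard and lets the player trigger an easter egg.
; A new puzzle turn closes the UI, then a timeline raises the now-visible keyboard along Z.
; When it finishes, control returns to the player, the pure-interaction camera takes over, and the terminal swaps to a lit mesh.
; Each tick, the player's easter-egg trigger flag is on only while interacting in that mode.
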(event Custom|Load%20Animation
  (Rendering|SetVisibility (Variables|Default|GetKeyboard) true false)
  (Variables|Default|SetDefault%20Keyboard%20Location (Transformation|GetWorldLocation (Variables|Default|GetKeyboard)))
  (bind _z_axis (Timeline|Animation PlayFromStart)
    (:Update
      (Transformation|SetWorldLocation (Variables|Default|GetKeyboard) (Math|Vector|MakeVector (.x (Variables|Default|GetDefault%20Keyboard%20Location)) (.y (Variables|Default|GetDefault%20Keyboard%20Location)) (+ (* _z_axis 25.0) (.z (Variables|Default|GetDefault%20Keyboard%20Location)))) false false))
    (:Finished
      (CallFunction|ManuallySwitchBacktoPlayer)
      (Components|Activation|SetActive (Variables|Default|GetCamera) false false)
      (Components|Activation|SetActive (Variables|Default|GetPure%20Interaction%20Camera) true false)
      (Variables|Default|SetPure%20Interaction true)
      (Components|StaticMesh|SetStaticMesh (Variables|Default|GetTerminal) (Variables|Default|GetLit%20Mesh)))))

(event EventBeginPlay
  (|CallParentFunction) ; This node is disabled and will not be called.\nDrag off pins to build functionality.
)

(event Collision|EventActorBeginOverlap
  (params (OtherActor :type Actor%20Object%20Reference)))

(event EventTick
  (params (DeltaSeconds :type Float%20%28single-precision%29))
  (bind _player_ref (Variables|Default|GetPlayer%20Ref)
    (:then
      (if (and (Variables|Default|GetPure%20Interaction) (Variables|Default|Getbeing%20interacted))
        (Variables|/Game/Characters/BP_ThirdPersonCharacter_Base.BP_ThirdPersonCharacter_Base_C|SetCan%20trigger%20easter-egg _player_ref true)
        (else
          (Variables|/Game/Characters/BP_ThirdPersonCharacter_Base.BP_ThirdPersonCharacter_Base_C|SetCan%20trigger%20easter-egg _player_ref false))))
    (:else)))

(event EventNewTurnOfPuzzle
  (CallFunction|ManuallyCloseUI)
  (CallFunction|LoadAnimation))

(fn ConstructionScript
  (|CallParentFunction))