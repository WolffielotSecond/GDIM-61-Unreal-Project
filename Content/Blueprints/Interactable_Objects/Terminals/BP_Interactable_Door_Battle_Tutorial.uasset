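; An interactable battle-tutorial door that holds back a player who has entered the safe room but has no knife.
; Its Interact event does nothing unless Solved is set, then checks the safe room and knife flags on PlayerRef.
; A knifeless player who has entered the safe room gets a look-at prompt message from DT_Look_At_Battle_Tutorial_Door, while all others trigger SolvedInteraction.
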(event EventBeginPlay
  (|CallParentFunction) ; This node is disabled and will not be called.\nDrag off pins to build functionality.
)

(event Collision|EventActorBeginOverlap
  (params (OtherActor :type Actor%20Object%20Reference))
  (|CallParentFunction OtherActor) ; This node is disabled and will not be called.\nDrag off pins to build functionality.
)

(event EventTick
  (params (DeltaSeconds :type Float%20%28single-precision%29))
  (|CallParentFunction DeltaSeconds) ; This node is disabled and will not be called.\nDrag off pins to build functionality.
)

(event EventInteract
  (if (Variables|Default|GetSolved?)
    (if (Variables|/Game/Characters/BP_ThirdPersonCharacter_Base.BP_ThirdPersonCharacter_Base_C|Gethas%20entered%20safe%20room (Variables|Default|GetPlayer%20Ref))
      (if (Variables|/Game/Characters/BP_ThirdPersonCharacter_Base.BP_ThirdPersonCharacter_Base_C|GetHas%20Knife (Variables|Default|GetPlayer%20Ref))
        (CallFunction|SolvedInteraction)
        (else
          (Class|BPIPlayerInterface|LookatPromptPlay(Message) (Game|GetPlayerCharacter 0) "/Game/Dialogs/Look_At_Dialogs/DT_Look_At_Battle_Tutorial_Door.DT_Look_At_Battle_Tutorial_Door")))
      (else
        (CallFunction|SolvedInteraction)))))

(fn ConstructionScript
  (|CallParentFunction))