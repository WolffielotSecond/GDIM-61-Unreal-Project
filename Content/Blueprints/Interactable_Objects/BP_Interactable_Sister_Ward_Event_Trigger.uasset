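; An interactable event trigger for the Sister Ward that plays a dialog, then has Meimei transform.
; Interact disables the sphere collision, asks the player to create a dialog widget from DT_Sister_Ward, and sets a local open flag.
; While that flag is set, Tick polls the player's dialog state and, once it closes, clears the flag and calls Transform on the Meimei reference.
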(event EventBeginPlay
  (|CallParentFunction) ; This node is disabled and will not be called.\nDrag off pins to build functionality.
)

(event Collision|EventActorBeginOverlap
  (params (OtherActor :type Actor%20Object%20Reference)))

(event EventTick
  (params (DeltaSeconds :type Float%20%28single-precision%29))
  (if (Variables|Default|GetDialog%20Widget%20Opened)
    (if (not (Variables|/Game/Characters/BP_ThirdPersonCharacter_Base.BP_ThirdPersonCharacter_Base_C|GetDialog%20Widget%20Opened (Variables|Default|GetPlayer%20Ref)))
      (Variables|Default|SetDialog%20Widget%20Opened false)
      (Default|Transform (Variables|Default|GetMeimei%20Ref)))))

(event EventInteract
  (Collision|SetCollisionEnabled (Variables|Default|GetSphere%20Collision) "NoCollision")
  (Default|CreateDialogWidget (Variables|Default|GetPlayer%20Ref) "/Game/Dialogs/Sister_Related/DT_Sister_Ward.DT_Sister_Ward")
  (Variables|Default|SetDialog%20Widget%20Opened true))

(fn ConstructionScript
  (|CallParentFunction))