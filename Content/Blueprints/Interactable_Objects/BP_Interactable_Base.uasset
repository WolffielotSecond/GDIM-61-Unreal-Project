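; Base Blueprint for interactable objects, showing a world interaction prompt widget for the player.
; On BeginPlay it creates a WB_Interact widget and sets its displayed information from the interaction type.
; A sphere collision notifies overlapping actors to register or remove the object and caches the player reference, while ShowUI and HideUI toggle the widget's visibility.
; Description text and key item ID functions return empty defaults, apparently as hooks for child classes.
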(event OnComponentBeginOverlap(SphereCollision)
  (params (OverlappedComponent :type Primitive%20Component%20Object%20Reference) (OtherActor :type Actor%20Object%20Reference) (OtherComp :type Primitive%20Component%20Object%20Reference) (OtherBodyIndex :type Integer) (bFromSweep :type Boolean) (SweepResult :type Hit%20Result%20Structure%20%28by%20ref%29))
  (Class|BPIPlayerInterface|GetInteractableObject(Message) OtherActor self)
  (Variables|Default|GetPlayer%20Ref
    (:then)
    (:else
      (bind _asbp_third_person_character_base (Utilities|Casting|CastToBP_ThirdPersonCharacter_Base OtherActor))
      (Variables|Default|SetPlayer%20Ref _asbp_third_person_character_base))))

(event OnComponentEndOverlap(SphereCollision)
  (params (OverlappedComponent :type Primitive%20Component%20Object%20Reference) (OtherActor :type Actor%20Object%20Reference) (OtherComp :type Primitive%20Component%20Object%20Reference) (OtherBodyIndex :type Integer))
  (Class|BPIPlayerInterface|RemoveInteractableObject(Message) OtherActor self)
  (if (Actor|ActorHasTag OtherActor "Player")
    (Variables|Widget|SetShow%20widget false)
    (Rendering|SetVisibility (Variables|Default|GetInteraction%20Widget) false false)))

(event EventBeginPlay
  (bind _returnvalue (UserInterface|CreateWidget "/Game/UI/Interactable_Object_UI/WB_Interact.WB_Interact_C"))
  (bind _output_get (Variables|Widget|SetInteraction%20Widget%20Ref _returnvalue))
  (UserInterface|SetWidget (Variables|Default|GetInteraction%20Widget) _output_get)
  (Default|SetDisplayedInformation _output_get (Variables|ForTuning|GetInteraction%20Type)))

(event EventShowUI
  (Variables|Widget|SetShow%20widget true)
  (Rendering|SetVisibility (Variables|Default|GetInteraction%20Widget) true false))

(event EventHideUI
  (Variables|Widget|SetShow%20widget false)
  (Rendering|SetVisibility (Variables|Default|GetInteraction%20Widget) false false))

(fn ConstructionScript)

(fn GetInteractioDescriptionText
  (return ""))

(fn ReturnKeyItemID
  (return "None"))