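; Vertical-slice path blocker that opens once all of its related tumors are cleared.
; Each TumorCleared call decrements the count set on BeginPlay from TumorsRelated, triggers a save game message and starts a cutscene at zero.
; The timed cutscene disables input, blends to its own camera, hides the cube, then uses black fades to show an airshaft camera and organ-restarted message before restoring player view and control.
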(event Custom|Check%20Remaining%20Number%20of%20Tumors
  (if (<= (Variables|Default|GetNumber%20of%20tumors) 0)
    (CallFunction|CameraMovementAnimation)))

(event Custom|Tumor%20Cleared
  (Math|Integer|DecrementInt (Variables|Default|GetNumber%20of%20tumors)
    (:%20%20
      (CallFunction|CheckRemainingNumberOfTumors)
      (Class|BPIGamecontroller|SaveGame(Message) (Game|GetPlayerController 0)))))

(event Custom|Camera%20Movement%20Animation
  (bind _asbp_third_person_character_base (Utilities|Casting|CastToBP_ThirdPersonCharacter_Base (Game|GetPlayerCharacter 0)))
  (Variables|Default|SetPlayer%20Ref _asbp_third_person_character_base)
  (Input|DisableInput (Game|GetPlayerCharacter 0) (Game|GetPlayerController 0))
  (Game|Player|SetViewTargetwithBlend (Game|GetPlayerController 0) (Variables|Default|Getcamera%20self) 1.5 "VTBlend_Linear" 0.0 false)
  (Utilities|FlowControl|Delay 2.5)
  (CallFunction|BreakItself)
  (Utilities|FlowControl|Delay 1.5)
  (bind _returnvalue (UserInterface|CreateWidget "/Game/UI/WB_Death_Black.WB_Death_Black_C" (Game|GetPlayerController 0)))
  (bind _output_get (Variables|Default|SetBlack%20Out%20Widget _returnvalue))
  (UserInterface|Viewport|AddtoViewport _output_get 0)
  (Default|PlayBlackAnimation _output_get)
  (Utilities|FlowControl|Delay 0.6)
  (Game|Player|SetViewTargetwithBlend (Game|GetPlayerController 0) (Variables|Default|Getcamera%20airshaft) 0.0 "VTBlend_Linear" 0.0 false)
  (Utilities|FlowControl|Delay 0.5)
  (Default|PlayBlackOut (Variables|Default|GetBlack%20Out%20Widget))
  (Utilities|FlowControl|Delay 1.6)
  (Class|BPIGamecontroller|VerticleSliceOrganRestarted(Message) (Game|GetPlayerController 0))
  (Utilities|FlowControl|Delay 2.0)
  (Default|PlayBlackAnimation (Variables|Default|GetBlack%20Out%20Widget))
  (Utilities|FlowControl|Delay 0.6)
  (Game|Player|SetViewTargetwithBlend (Game|GetPlayerController 0) (Variables|/Game/Characters/BP_ThirdPersonCharacter_Base.BP_ThirdPersonCharacter_Base_C|GetCamera%20Actor%20Reference (Variables|Default|GetPlayer%20Ref)) 0.0 "VTBlend_Linear" 0.0 false)
  (Default|PlayBlackOut (Variables|Default|GetBlack%20Out%20Widget))
  (Utilities|FlowControl|Delay 0.6)
  (Input|EnableInput (Game|GetPlayerCharacter 0) (Game|GetPlayerController 0))
  (Widget|RemovefromParent (Variables|Default|GetBlack%20Out%20Widget)))

(event Custom|Break%20itself
  (Rendering|SetVisibility (Variables|Default|GetCube) false false))

(event EventBeginPlay
  (Variables|Default|SetNumber%20of%20tumors (Utilities|Array|Length (Variables|Default|GetTumors%20Related))))

(fn ConstructionScript)