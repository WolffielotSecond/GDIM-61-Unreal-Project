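; Base interactable terminal for puzzles, whose child classes override the solved animation, solved interaction and new puzzle turn events.
; Interacting while unsolved hides the player mesh, blends the view to the terminal, blocks inventory and, unless PureInteraction, opens the interaction menu.
; Engaging it either starts a new turn on multiple-use terminals or marks it solved.
; Manual events close the UI and restore the player's camera and state.
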(event Custom|Play%20Terminal%20Solved%20Animation
  ;[0.15 0.15 0.15 0.5] 子类只需override这仨
)

(event Custom|New%20Turn%20of%20Puzzle
  ;[0.15 0.15 0.15 0.5] 子类只需override这仨
  ;;[0.15 0.15 0.15 0.5] 这个需要改is multiple use terminals和item Received Name
)

(event Custom|Manually%20Close%20UI
  (bind _returnvalue (Game|GetPlayerController 0))
  (Widget|RemovefromParent (Variables|/Game/Characters/BP_ThirdPersonCharacter_Base.BP_ThirdPersonCharacter_Base_C|GetInteraction%20Menu (Variables|Default|GetPlayer%20Ref)))
  (Input|SetInputModeGameOnly _returnvalue false)
  (Variables|/Script/Engine.PlayerController|SetbShowMouseCursor _returnvalue false))

(event Custom|Manually%20Switch%20back%20to%20player
  (bind _player_ref (Variables|Default|GetPlayer%20Ref))
  (Rendering|SetVisibility (Variables|/Script/Engine.Character|GetMesh (Variables|Default|GetPlayer%20Ref)) true true)
  (Variables|/Game/Characters/BP_ThirdPersonCharacter_Base.BP_ThirdPersonCharacter_Base_C|SetCan%20Open%20Inventory _player_ref true)
  (Variables|/Game/Characters/BP_ThirdPersonCharacter_Base.BP_ThirdPersonCharacter_Base_C|SetInteraction%20UI%20Opened _player_ref false)
  (Variables|Default|Setbeing%20interacted false)
  (Game|Player|SetViewTargetwithBlend (Game|GetPlayerController 0) (Variables|/Game/Characters/BP_ThirdPersonCharacter_Base.BP_ThirdPersonCharacter_Base_C|GetCamera%20Actor%20Reference _player_ref) 0.0 "VTBlend_Linear" 0.0 false))

(event Custom|Solved%20Interaction
  ;[0.15 0.15 0.15 0.5] 子类只需override这仨
)

(event EventBeginPlay
  (|CallParentFunction))

(event EventTerminalIngaged
  (if (Variables|Default|GetIs%20Multiple%20Use%20Terminals)
    (CallFunction|NewTurnOfPuzzle)
    (else
      (Variables|Default|SetSolved? true)
      (CallFunction|PlayTerminalSolvedAnimation))))

(event EventStopBeingInteracted
  (Variables|Default|Setbeing%20interacted false))

(event EventInteract
  (bind _player_ref (Variables|Default|GetPlayer%20Ref))
  (if (Variables|Default|GetSolved?)
    (CallFunction|SolvedInteraction)
    (else
      (Variables|Default|Setbeing%20interacted true)
      (Rendering|SetVisibility (Variables|/Script/Engine.Character|GetMesh _player_ref) false true)
      (Variables|/Game/Characters/BP_ThirdPersonCharacter_Base.BP_ThirdPersonCharacter_Base_C|SetInteraction%20UI%20Opened _player_ref true)
      (Game|Player|SetViewTargetwithBlend (Game|GetPlayerController 0) self 0.0 "VTBlend_Linear" 0.0 false)
      (Variables|/Game/Characters/BP_ThirdPersonCharacter_Base.BP_ThirdPersonCharacter_Base_C|SetCan%20Open%20Inventory (Variables|Default|GetPlayer%20Ref) false)
      (if (not (Variables|Default|GetPure%20Interaction))
        (Default|OpenInteractionMenuUI (Variables|Default|GetPlayer%20Ref))))))

(fn ConstructionScript
  (|CallParentFunction))

(fn ReturnKeyItemID
  (return (Variables|Default|GetItem%20Received%20Name)))

(fn GetInteractioDescriptionText
  (return (Variables|Default|GetInteraction%20Description)))