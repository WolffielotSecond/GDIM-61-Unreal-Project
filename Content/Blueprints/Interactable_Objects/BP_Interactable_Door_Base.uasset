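; Base interactable door that swings open and closed with timelines and streams in the next level when its puzzle is solved.
; Solving an interaction toggles the door unless it is mid-swing, switching collision off while it moves or stands open.
; A player leaving the auto-close volume shuts it.
; The terminal-solved sequence closes the UI, loads the unlocking level, and plays chained key insert, turn and withdraw animations before returning control to the player.
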(event OnComponentEndOverlap(AutoCloseDoorCollision)
  (params (OverlappedComponent :type Primitive%20Component%20Object%20Reference) (OtherActor :type Actor%20Object%20Reference) (OtherComp :type Primitive%20Component%20Object%20Reference) (OtherBodyIndex :type Integer))
  (if (Actor|ActorHasTag OtherActor "Player")
    (if (Variables|Default|GetIs%20Opened)
      (CallFunction|CloseDoor))))

(event Custom|Play%20Close%20Animation
  (Variables|Default|SetDoor%20Playing%20Open/%20Close%20Anim true)
  (Collision|SetCollisionEnabled (Variables|Default|GetDoor) "NoCollision")
  (bind _percentage (Timeline|Door%20Close PlayFromStart)
    (:Update
      (Transformation|SetRelativeRotation (Variables|Default|GetDoor) (Math|Rotator|MakeRotator 0.0 0.0 (* _percentage 9e+01)) false false))
    (:Finished
      (Variables|Default|SetDoor%20Playing%20Open/%20Close%20Anim false)
      (Collision|SetCollisionEnabled (Variables|Default|GetDoor) "QueryAndPhysics"))))

(event Custom|Play%20Open%20Animation
  (Variables|Default|SetDoor%20Playing%20Open/%20Close%20Anim true)
  (Collision|SetCollisionEnabled (Variables|Default|GetDoor) "NoCollision")
  (bind _percentage (Timeline|Door%20Open PlayFromStart)
    (:Update
      (Transformation|SetRelativeRotation (Variables|Default|GetDoor) (Math|Rotator|MakeRotator 0.0 0.0 (+ (* _percentage 9e+01) 0.0)) false false))
    (:Finished
      (Variables|Default|SetDoor%20Playing%20Open/%20Close%20Anim false)
      (Collision|SetCollisionEnabled (Variables|Default|GetDoor) "QueryAndPhysics"))))

(event Custom|Load%20Next%20Level
  (Game|LoadStreamLevel(byName) (Variables|Default|GetUnlocking%20Level) true))

(event Custom|Close%20Door
  (Variables|Default|SetIs%20Opened false)
  (CallFunction|PlayCloseAnimation)
  (Collision|SetCollisionEnabled (Variables|Default|GetDoor%20Collision) "QueryAndPhysics"))

(event Custom|Open%20Door
  (Variables|Default|SetIs%20Opened true)
  (CallFunction|PlayOpenAnimation)
  (Collision|SetCollisionEnabled (Variables|Default|GetDoor%20Collision) "NoCollision"))

(event Collision|EventActorBeginOverlap
  (params (OtherActor :type Actor%20Object%20Reference)))

(event EventTick
  (params (DeltaSeconds :type Float%20%28single-precision%29)))

(event EventPlayTerminalSolvedAnimation
  (bind _key (Variables|Default|GetKey))
  (CallFunction|ManuallyCloseUI)
  (CallFunction|LoadNextLevel)
  (Rendering|SetVisibility _key true false)
  (Transformation|SetRelativeRotation _key "-90.000000,0.000000,0.000000" false false)
  ;[0.15 0.15 0.15 0.5] 22变4.5
  (Transformation|SetRelativeLocation _key "52.300000,22.000000,-11.000000" false false)
  (bind _y_axis (Timeline|Key%20In PlayFromStart)
    (:Update
      (Transformation|SetRelativeLocation (Variables|Default|GetKey) (Math|Vector|MakeVector 52.3 (+ (* _y_axis -17.5) 22.0) -11.0) false false))
    (:Finished
      (bind _rotation (Timeline|Rotate%20Key PlayFromStart)
        (:Update
          (Transformation|SetRelativeRotation (Variables|Default|GetKey) (Math|Rotator|MakeRotator 0.0 _rotation 0.0) false false))
        (:Finished
          (bind _y_axis_2 (Timeline|Finish PlayFromStart)
            (:Update
              (Transformation|SetRelativeLocation (Variables|Default|GetKey) (Math|Vector|MakeVector 52.3 (+ (* _y_axis_2 17.5) 4.5) -11.0) false false))
            (:Finished
              (CallFunction|ManuallySwitchBacktoPlayer)
              (Rendering|SetVisibility (Variables|Default|GetKey) false false))))))))

(event EventSolvedInteraction
  (bind _door_collision (Variables|Default|GetDoor%20Collision))
  (if (not (Variables|Default|GetDoor%20Playing%20Open/%20Close%20Anim))
    (if (Variables|Default|GetIs%20Opened)
      (Variables|Default|SetIs%20Opened false)
      (CallFunction|PlayCloseAnimation)
      (Collision|SetCollisionEnabled _door_collision "QueryAndPhysics")
      (else
        (Variables|Default|SetIs%20Opened true)
        (CallFunction|PlayOpenAnimation)
        (Collision|SetCollisionEnabled _door_collision "NoCollision")))))

(event EventBeginPlay
  (Rendering|SetVisibility (Variables|Default|GetKey) false false))

(fn ConstructionScript
  (|CallParentFunction))