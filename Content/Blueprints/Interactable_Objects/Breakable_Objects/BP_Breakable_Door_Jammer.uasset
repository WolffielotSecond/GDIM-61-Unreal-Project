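; Breakable door jammer that the player clears, with a built-in tutorial prompt about breaking vines with an attack.
; BreakWood asks the first player controller to save the game through an interface-style message, then destroys the actor.
; The PlayerTutorialActivator overlap checks for a Player-tagged actor holding a knife, then shows the left-mouse attack hint on the player character once.
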(event OnComponentBeginOverlap(PlayerTutorialActivator)
  (params (OverlappedComponent :type Primitive%20Component%20Object%20Reference) (OtherActor :type Actor%20Object%20Reference) (OtherComp :type Primitive%20Component%20Object%20Reference) (OtherBodyIndex :type Integer) (bFromSweep :type Boolean) (SweepResult :type Hit%20Result%20Structure%20%28by%20ref%29))
  (if (Actor|ActorHasTag OtherActor "Player")
    (bind _has_knife (Class|BPIPlayerInterface|GetHasKnife(Message) OtherActor))
    (if _has_knife
      (Utilities|FlowControl|DoOnce false
        (:Completed
          (Class|BPIPlayerInterface|PlayTutorialMessage(Message) (Game|GetPlayerCharacter 0) "Attack with LMB to Break Vines" false 0.0))))))

(event EventBeginPlay
  (|CallParentFunction) ; This node is disabled and will not be called.\nDrag off pins to build functionality.
)

(event Collision|EventActorBeginOverlap
  (params (OtherActor :type Actor%20Object%20Reference)))

(event EventTick
  (params (DeltaSeconds :type Float%20%28single-precision%29)))

(event EventBreakWood
  (Class|BPIGamecontroller|SaveGame(Message) (Game|GetPlayerController 0))
  (Actor|DestroyActor))

(fn ConstructionScript
  (|CallParentFunction))