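; BPC_Entity_Stats is a component that tracks health and tenacity (poise) for its BP_EnemyBase owner.
; Damage subtracts from Health, and reaching zero only prints a debug string.
; Tenacity damage accumulates up to MaxTenacity, then triggers EnemyStunned on the cached owner and resets to zero.
; Tenacity does not build while the enemy is in its stunned state.
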(event Custom|是否破刃击晕
  (if (>= (Variables|Default|GetTenacity) (Variables|Default|GetMax%20Tenacity))
    (Default|EnemyStunned (Variables|Default|GetEnemy%20Self%20Ref))
    (Variables|Default|SetTenacity 0.0)))

(event Custom|扣血
  (params (Health%20Lost :type Float%20%28double-precision%29))
  ;[0.15 0.15 0.15 0.5] 扣血是做减法
  (Variables|Default|SetHealth (- (Variables|Default|GetHealth) Health%20Lost))
  (CallFunction|是否撕掉))

(event Custom|扣韧
  (params (Tenacity%20Lost :type Float%20%28double-precision%29))
  ;[0.15 0.15 0.15 0.5] tenacity是从0累加到max tenacity的而不是做减法,并且在stunned state不会累加条
  (if (Utilities|Enum|NotEqual(Enum) (Variables|/Game/Enemies/BP_EnemyBase.BP_EnemyBase_C|GetEnemy%20State (Variables|Default|GetEnemy%20Self%20Ref)) "NewEnumerator4")
    (Variables|Default|SetTenacity (+ (Variables|Default|GetTenacity) Tenacity%20Lost))
    (CallFunction|是否破刃击晕)))

(event Custom|是否撕掉
  (if (<= (Variables|Default|GetHealth) 0.0)
    (Development|PrintString "饿")))

(event EventBeginPlay
  (bind _asbp_enemy_base (Utilities|Casting|CastToBP_EnemyBase (Components|GetOwner)))
  (Variables|Default|SetEnemy%20Self%20Ref _asbp_enemy_base))