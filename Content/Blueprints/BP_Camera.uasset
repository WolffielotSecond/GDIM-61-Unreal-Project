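; Player-following camera for a 3D platformer that registers itself in the game instance and also drives enemy auto-targeting.
; Tick eases toward the player with damped X movement, tilts pitch with depth and adds a clamped mouse free-look offset with cosine-squared resistance.
; An overlap volume collects tagged enemies, passing the nearest to the player with lock/unlock messages.
; It also handles death/respawn exposure effects and eased spring-arm length and side-offset changes.
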(event EventBeginPlay
  (bind _springarm (Variables|Default|GetSpringArm))
  (bind _returnvalue (Transformation|GetWorldLocation _springarm))
  (Utilities|Struct|SetmembersinPostProcessSettings (Variables|/Script/Engine.CameraComponent|GetPostProcessSettings (Variables|Default|GetCamera)) 1.0)
  (Variables|/Script/Engine.SpringArmComponent|SetbDoCollisionTest (Variables|Default|GetSpringArm) false)
  (bind _player_reference (Variables|Default|GetPlayer%20Reference)
    (:then
      (Variables|Default|SetDefault%20Actor%20Location (Transformation|GetWorldLocation (Variables|/Game/Characters/BP_ThirdPersonCharacter_Base.BP_ThirdPersonCharacter_Base_C|GetCamera%20Prompt _player_reference)))
      (Variables|Default|SetCenter%20Camera%20Location (Math|Vector|MakeVector (.x (Transformation|GetWorldLocation (Variables|Default|GetCamera))) (.y _returnvalue) (.z _returnvalue)))
      (bind _asbpinstance_platformer_3d (Utilities|Casting|CastToBPInstance_Platformer_3D (Game|GetGameInstance)))
      (Variables|/Game/Blueprints/BPInstance_Platformer_3D.BPInstance_Platformer_3D_C|SetCamera%20Ref _asbpinstance_platformer_3d self))
    (:else
      (Development|PrintString "Hello"))))

(event EventTick
  (params (DeltaSeconds :type Float%20%28single-precision%29))
  (bind _returnvalue (Transformation|GetActorLocation))
  (bind _default_actor_location (Variables|Default|GetDefault%20Actor%20Location))
  (bind _springarm (Variables|Default|GetSpringArm))
  (bind _default_actor_location_2 (Variables|Default|GetDefault%20Actor%20Location))
  (bind _player_reference (Variables|Default|GetPlayer%20Reference))
  (bind _camera (Variables|Default|GetCamera))
  (bind _springarm_2 (Variables|Default|GetSpringArm))
  (bind _returnvalue_2 (Transformation|GetWorldLocation _springarm))
  (bind _returnvalue_3 (Transformation|GetActorLocation _player_reference))
  (bind _returnvalue_4 (Transformation|GetWorldLocation _springarm_2))
  (bind _postprocesssettings (Variables|/Script/Engine.CameraComponent|GetPostProcessSettings _camera))
  (Utilities|FlowControl|Sequence
    (:then_0
      ;[0.15 0.15 0.15 0.5] 先创建一个变量限制是否跟随
      (if (Variables|Default|GetCamera%20Should%20Follow%20Player)
        ;[0.15 0.15 0.15 0.5] 防止玩家没被赋值时运行后面的东西然后报错
        (bind _player_reference_2 (Variables|Default|GetPlayer%20Reference)
          (:then
            ;[0.15 0.15 0.15 0.5] 摄像机整个actor跟随玩家
            (Transformation|SetActorLocation (Math|Interpolation|VInterpTo (Transformation|GetActorLocation) (Math|Vector|MakeVector (+ (/ (- (.x (Transformation|GetWorldLocation (Variables|/Game/Characters/BP_ThirdPersonCharacter_Base.BP_ThirdPersonCharacter_Base_C|GetCamera%20Prompt _player_reference_2))) (.x _default_actor_location_2)) 5.0) (.x _default_actor_location_2)) (.y (Transformation|GetWorldLocation (Variables|/Game/Characters/BP_ThirdPersonCharacter_Base.BP_ThirdPersonCharacter_Base_C|GetCamera%20Prompt _player_reference_2))) (.z (Transformation|GetWorldLocation (Variables|/Game/Characters/BP_ThirdPersonCharacter_Base.BP_ThirdPersonCharacter_Base_C|GetCamera%20Prompt _player_reference_2)))) (Utilities|Time|GetWorldDeltaSeconds) 7.5) false false)
            ;[0.15 0.15 0.15 0.5] 赋值默认镜头位置确保鼠标让镜头晃动不出错
            (Variables|Default|SetCenter%20Camera%20Location (Math|Vector|MakeVector (- (.x _returnvalue_4) (Variables|/Script/Engine.SpringArmComponent|GetTargetArmLength _springarm_2)) (.y _returnvalue_4) (.z _returnvalue_4))))
          (:else))
        (else
          (bind _player_reference_3 (Variables|Default|GetPlayer%20Reference)
            (:then
              (Transformation|SetActorLocation (Math|Interpolation|VInterpTo (Transformation|GetActorLocation) (Math|Vector|MakeVector (+ (/ (- (.x (Transformation|GetWorldLocation (Variables|/Game/Characters/BP_ThirdPersonCharacter_Base.BP_ThirdPersonCharacter_Base_C|GetCamera%20Prompt _player_reference_3))) (.x _default_actor_location)) 5.0) (.x _default_actor_location)) (.y _returnvalue) (.z _returnvalue)) (Utilities|Time|GetWorldDeltaSeconds) 7.5) false false)
              (Variables|Default|SetCenter%20Camera%20Location (Math|Vector|MakeVector (- (.x _returnvalue_2) (Variables|/Script/Engine.SpringArmComponent|GetTargetArmLength _springarm)) (.y _returnvalue_2) (.z _returnvalue_2))))
            (:else)))))
    (:then_1
      (if (Variables|FreeLook|GetCamera%20Is%20Moving)
        (Transformation|SetWorldLocation (Variables|Default|GetCamera) (+ (Variables|Default|GetCamera%20Offset%20Vector) (Variables|Default|GetCenter%20Camera%20Location)) false false)))
    (:then_2
      (Transformation|SetWorldLocation (Variables|Default|Get自动索敌圈) (Math|Vector|MakeVector (.x _returnvalue_3) (.y (Transformation|GetWorldLocation (Variables|Default|GetCamera))) (.z _returnvalue_3)) false false))
    (:then_3
      (CallFunction|FindNearestEnemy))
    (:then_4
      (Transformation|SetRelativeRotation (Variables|Default|GetCamera) (Math|Rotator|MakeRotator 0.0 (Math|Float|Lerp -17.5 -1e+01 (/ (+ (/ (- (.x (Transformation|GetActorLocation)) (.x (Variables|Default|GetDefault%20Actor%20Location))) 5.0) 25.0) 75.0)) 0.0) false false))
    (:then_5
      (if (Variables|Default|GetShould%20Play%20Death%20Respawn%20Exposure)
        (Utilities|Struct|SetmembersinPostProcessSettings _postprocesssettings (Math|Interpolation|FInterpTo (Utilities|Struct|BreakPostProcessSettings _postprocesssettings) 1.0 (Utilities|Time|GetWorldDeltaSeconds) 2.0))
        (if (Math|Float|NearlyEqual(Float) (Utilities|Struct|BreakPostProcessSettings (Variables|/Script/Engine.CameraComponent|GetPostProcessSettings (Variables|Default|GetCamera))) 1.0 0.08)
          (Variables|Default|SetShould%20Play%20Death%20Respawn%20Exposure false)
          (Variables|/Game/Characters/BP_ThirdPersonCharacter_Base.BP_ThirdPersonCharacter_Base_C|Setis%20playing%20respawn%20animation (Variables|Default|GetPlayer%20Reference) false))))
    (:then_6
      (CallFunction|相机往外拉长逻辑))))

(event Custom|Free%20Camera%20Movement
  (params (Action%20Value%20X :type Float%20%28double-precision%29) (Action%20Value%20Y :type Float%20%28double-precision%29) (Max%20X :type Float%20%28double-precision%29) (Max%20Y :type Float%20%28double-precision%29))
  ;[0.15 0.15 0.15 0.5] 存储最高鼠标能移动的角度
  (Variables|FreeLook|SetMax%20X Max%20X)
  (Variables|FreeLook|SetMax%20Y Max%20Y)
  (Variables|FreeLook|SetAccumulated%20X (Math|Float|Clamp(Float) (+ (Variables|FreeLook|GetAccumulated%20X) (* Action%20Value%20X (FreeLook|CalculateFreeCameraMovementResistance (Variables|FreeLook|GetAccumulated%20X) (Variables|FreeLook|GetMax%20X) Action%20Value%20X))) (* (Variables|FreeLook|GetMax%20X) -1.0) (Variables|FreeLook|GetMax%20X)))
  (Variables|FreeLook|SetAccumulated%20Y (Math|Float|Clamp(Float) (+ (Variables|FreeLook|GetAccumulated%20Y) (* Action%20Value%20Y (FreeLook|CalculateFreeCameraMovementResistance (Variables|FreeLook|GetAccumulated%20Y) (Variables|FreeLook|GetMax%20Y) Action%20Value%20Y))) (* (Variables|FreeLook|GetMax%20Y) -1.0) (Variables|FreeLook|GetMax%20Y)))
  ;[0.15 0.15 0.15 0.5] 赋值offset用于计算最终相机位置
  (Variables|Default|SetCamera%20Offset%20Vector (* (Math|Vector|MakeVector 0.0 (Variables|FreeLook|GetAccumulated%20X) (* (Variables|FreeLook|GetAccumulated%20Y) -1.0)) 1e+01)))

(event OnComponentBeginOverlap(自动索敌圈)
  (params (OverlappedComponent :type Primitive%20Component%20Object%20Reference) (OtherActor :type Actor%20Object%20Reference) (OtherComp :type Primitive%20Component%20Object%20Reference) (OtherBodyIndex :type Integer) (bFromSweep :type Boolean) (SweepResult :type Hit%20Result%20Structure%20%28by%20ref%29))
  (if (Actor|ActorHasTag OtherActor "Enemy")
    (Utilities|Array|Add (Variables|AutoLock|GetEnemies) OtherActor)))

(event OnComponentEndOverlap(自动索敌圈)
  (params (OverlappedComponent :type Primitive%20Component%20Object%20Reference) (OtherActor :type Actor%20Object%20Reference) (OtherComp :type Primitive%20Component%20Object%20Reference) (OtherBodyIndex :type Integer))
  (bind _enemies (Variables|AutoLock|GetEnemies))
  (if (Actor|ActorHasTag OtherActor "Enemy")
    (Utilities|IsValid OtherActor
      (:Is%20Valid
        (Utilities|Array|RemoveIndex _enemies (Utilities|Array|FindItem _enemies OtherActor))))))

(event Custom|Eye%20Death%20Effect
  (params (Exposed%20Seconds :type Float%20%28double-precision%29))
  (Utilities|Struct|SetmembersinPostProcessSettings (Variables|/Script/Engine.CameraComponent|GetPostProcessSettings (Variables|Default|GetCamera)) (+ (* Exposed%20Seconds 28.0) 1.0)))

(event Custom|相机往外拉长逻辑
  (bind _springarm (Variables|Default|GetSpringArm))
  (bind _springarm_2 (Variables|Default|GetSpringArm))
  (bind _springarm_3 (Variables|Default|GetSpringArm))
  (bind _relativelocation (Variables|/Script/Engine.SceneComponent|GetRelativeLocation _springarm_3))
  (if (Variables|修改fov|Getcamera%20should放大fov)
    (Variables|/Script/Engine.SpringArmComponent|SetTargetArmLength _springarm_2 (Math|Interpolation|FInterpTo (Variables|/Script/Engine.SpringArmComponent|GetTargetArmLength _springarm_2) (Variables|修改fov|Gettarget%20spring%20arm%20length) (Utilities|Time|GetWorldDeltaSeconds) 1.0))
    (Transformation|SetRelativeLocation _springarm_3 (Math|Vector|MakeVector (.x _relativelocation) (Math|Interpolation|FInterpTo (.y _relativelocation) (Variables|修改fov|GetTarget%20Arm%20Y%20Location) (Utilities|Time|GetWorldDeltaSeconds) 1.0) (.z _relativelocation)) false false)
    (if (and (Math|Float|NearlyEqual(Float) (Variables|/Script/Engine.SpringArmComponent|GetTargetArmLength _springarm) (Variables|修改fov|Gettarget%20spring%20arm%20length) 0.08) (Math|Float|NearlyEqual(Float) (.y (Variables|/Script/Engine.SceneComponent|GetRelativeLocation _springarm)) (Variables|修改fov|GetTarget%20Arm%20Y%20Location) 0.08))
      (Variables|修改fov|Setcamera%20should放大fov false))))

(event Custom|Set%20Target%20FOV%20change%20values
  (params (Target%20Arm%20Length :type Float%20%28double-precision%29) (Target%20Arm%20Y%20Location :type Float%20%28double-precision%29))
  (Variables|修改fov|Settarget%20spring%20arm%20length Target%20Arm%20Length)
  (Variables|修改fov|SetTarget%20Arm%20Y%20Location Target%20Arm%20Y%20Location)
  (Variables|修改fov|Setcamera%20should放大fov true))

(fn ConstructionScript)

(fn CalculateFreeCameraMovementResistance
  (params (Current%20Value :type Float%20%28double-precision%29) (Maximum%20Value :type Float%20%28double-precision%29) (input%20Value :type Float%20%28double-precision%29))
  (bind _returnvalue (Math|Float|Absolute(Float) Current%20Value))
  (if (>= (* input%20Value Current%20Value) 0.0)
    ;[0.15 0.15 0.15 0.5] 情况1鼠标移动方向与目前累计数值符号相同时需要有减速处理
    (return (Math|Float|Square (Math|Trig|Cos(Degrees) (* (/ _returnvalue (* Maximum%20Value 2.0)) 1.8e+02))))
    (else
      ;[0.15 0.15 0.15 0.5] 情况2鼠标方向与累计数值符号相反则不必上来就减速，直接把已有数值和累计数值叠加然后用这个值来计算所需的阻力
      (return (Math|Float|Square (Math|Trig|Cos(Degrees) (* (/ _returnvalue (* (+ Maximum%20Value _returnvalue) 2.0)) 1.8e+02)))))))

(fn FindNearestEnemy
  (bind _player_reference (Variables|Default|GetPlayer%20Reference))
  (bind _player_reference_2 (Variables|Default|GetPlayer%20Reference))
  (Utilities|IsValid (Utilities|Array|Get(acopy) (Variables|AutoLock|GetEnemies))
    (:Is%20Valid
      (for _array_element (Variables|AutoLock|GetEnemies)
        (if (<= (Math|Vector|VectorLength (- (Transformation|GetWorldLocation (Variables|Default|Get自动索敌圈)) (Transformation|GetActorLocation _array_element))) (LocalVariables|GetNearest%20Location))
          (LocalVariables|SetNearest%20Actor _array_element)
          (LocalVariables|SetNearest%20Location (Math|Vector|VectorLength (- (Transformation|GetWorldLocation (Variables|Default|Get自动索敌圈)) (Transformation|GetActorLocation _array_element))))))
      (bind _auto_targeted_enemy (Variables|/Game/Characters/BP_ThirdPersonCharacter_Base.BP_ThirdPersonCharacter_Base_C|GetAuto%20Targeted%20Enemy _player_reference)
        (:then
          (if (not (== _auto_targeted_enemy (LocalVariables|GetNearest%20Actor)))
            (Class|BPIEnemy|OnTargetUnlock(Message) _auto_targeted_enemy)
            (bind _output_get (Variables|/Game/Characters/BP_ThirdPersonCharacter_Base.BP_ThirdPersonCharacter_Base_C|SetAuto%20Targeted%20Enemy _player_reference (LocalVariables|GetNearest%20Actor) :!label _label))
            (Class|BPIEnemy|OnTargetLock(Message) _output_get)))
        (:else
          (goto _label))))
    (:Is%20Not%20Valid
      (bind _auto_targeted_enemy_2 (Variables|/Game/Characters/BP_ThirdPersonCharacter_Base.BP_ThirdPersonCharacter_Base_C|GetAuto%20Targeted%20Enemy _player_reference_2)
        (:then
          (Class|BPIEnemy|OnTargetUnlock(Message) _auto_targeted_enemy_2)
          (Variables|/Game/Characters/BP_ThirdPersonCharacter_Base.BP_ThirdPersonCharacter_Base_C|SetAuto%20Targeted%20Enemy _player_reference_2 0))
        (:else)))))