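; BP_PressCtocrouch is a tutorial prompt that shows the crouch control matching the player's current input device.
; On BeginPlay it gets the custom game controller, binds its SwitchInput event to the controller's input-switch notification and applies the initial IsController state.
; A controller shows the Plane and PressRSToCrouch components, while other input shows only the TextRender, with both paths reusing the same visibility toggles.
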(event Custom|SwitchInput
  (params (Is%20Controller :type Boolean))
  (if Is%20Controller
    (Rendering|SetVisibility (Variables|Default|GetPlane) true false)
    (Rendering|SetVisibility (Variables|Default|GetPress%20RS%20to%20Crouch) true false)
    (Rendering|SetVisibility (Variables|Default|GetTextRender) false false)
    (else
      (Rendering|SetVisibility (Variables|Default|GetPlane) false false)
      (Rendering|SetVisibility (Variables|Default|GetPress%20RS%20to%20Crouch) false false)
      (Rendering|SetVisibility (Variables|Default|GetTextRender) true false))))

(event EventBeginPlay
  (bind _asbp_custom_game_controller (Utilities|Casting|CastToBP_Custom_GameController (Game|GetPlayerController 0)))
  (EventDispatchers|BindEventtoSwitch _asbp_custom_game_controller (delegate Custom|SwitchInput))
  (if (Variables|/Game/Blueprints/BP_Custom_GameController.BP_Custom_GameController_C|GetIs%20Controller _asbp_custom_game_controller)
    (Rendering|SetVisibility (Variables|Default|GetPlane) true false)
    (Rendering|SetVisibility (Variables|Default|GetPress%20RS%20to%20Crouch) true false)
    (Rendering|SetVisibility (Variables|Default|GetTextRender) false false)
    (else
      (Rendering|SetVisibility (Variables|Default|GetPlane) false false)
      (Rendering|SetVisibility (Variables|Default|GetPress%20RS%20to%20Crouch) false false)
      (Rendering|SetVisibility (Variables|Default|GetTextRender) true false))))

(fn ConstructionScript)